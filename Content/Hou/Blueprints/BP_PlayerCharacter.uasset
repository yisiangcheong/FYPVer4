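; First-person player character for a clue puzzle game, with movement, FOV zoom and pause menu.
; A camera trace drives clicks to grab "Pickup" objects via physics handle or message other actors, and throttled crosshair updates.
; While possessed, a velocity-driven step cycle times footstep sounds and three-axis head bob.
; When certain closing clues end, it sets the controller's ControllerForce flag and the book pawn's page.
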(event `Key|RightMouseButton`
  (params (Key :type "Key Structure"))
  ;[1 1 1] Right mouse click to zoom. It works by changing the camera FOV
  (:`Pressed`
    (bind (_direction _zoomalpha) (`Timeline|ZoomTimeline` :!label _label)
      (:`Update`
        (`CameraComponent.SetFieldOfView` (`self.FirstPersonCamera`) (`KismetMathLibrary.Lerp` (`self.DefaultFOV`) (`self.ZoomedFOV`) _zoomalpha)))))
  (:`Released`
    (goto _label :!via `Reverse`)))

(event `self.ReceiveBeginPlay`
  ;[1 1 1] Init
  (set `self.fpsCamOriginalRelLoc` (`SceneComponent.RelativeLocation` (`self.FirstPersonCamera`)))
  (set `self.NextStep` (+ (`self.StepCycle`) (`self.StepInterval`)))
  (set `self.DefaultFOV` (`CameraComponent.FieldOfView` (`self.FirstPersonCamera`)))
  (`KismetSystemLibrary.ExecuteConsoleCommand` "stat FPS" null))

(event `InputAxis|Turn` :overrideparent false
  (params (AxisValue :type "Float (single-precision)"))
  ;[1 1 1] Mouse Movement input
  (`self.AddControllerYawInput` AxisValue))

(event `InputAxis|MoveForward`
  (params (AxisValue :type "Float (single-precision)"))
  ;[1 1 1] Movement Keys Input
  (bind _output_get (set `self.ForwardInputAxisValue` AxisValue))
  (`self.AddMovementInput` (`KismetMathLibrary.GetForwardVector` (`self.GetControlRotation`)) _output_get))

(event `/Game/Hou/Blueprints/Interface_PuzzleUpdate.OnClosingClueEnded`
  (params (`Puzzle ID` :type "/Game/Hou/Blueprints/Enum_PuzzleID Enum" :default "NewEnumerator0"))
  (bind _returnvalue (`GameplayStatics.GetPlayerPawn` 0))
  (switch `/Game/Hou/Blueprints/Enum_PuzzleID` `Puzzle ID`
    (:`NewEnumerator1`
      (bind _asnew_player_controller (cast `/Game/Alex/NewPlayerController` (`GameplayStatics.GetPlayerController` 0)))
      ;[1 1 1] Book flips to page office
      (set `/Game/Alex/NewPlayerController.ControllerForce` true _asnew_player_controller)
      (bind _asbook_ui_pawn (cast `/Game/Alex/Prototype_Book/Book_UI_Pawn` _returnvalue))
      (set `/Game/Alex/Prototype_Book/Book_UI_Pawn.Page` 1 _asbook_ui_pawn))
    (:`NewEnumerator2`
      (bind _asnew_player_controller_2 (cast `/Game/Alex/NewPlayerController` (`GameplayStatics.GetPlayerController` 0)))
      (set `/Game/Alex/NewPlayerController.ControllerForce` true _asnew_player_controller_2)
      ;[1 1 1] Book flips to page bedroom
      (bind _asbook_ui_pawn_2 (cast `/Game/Alex/Prototype_Book/Book_UI_Pawn` _returnvalue))
      (set `/Game/Alex/Prototype_Book/Book_UI_Pawn.Page` 2 _asbook_ui_pawn_2))
    (:`NewEnumerator3`
      (bind _asnew_player_controller_3 (cast `/Game/Alex/NewPlayerController` (`GameplayStatics.GetPlayerController` 0)))
      (set `/Game/Alex/NewPlayerController.ControllerForce` true _asnew_player_controller_3)
      (bind _asbook_ui_pawn_3 (cast `/Game/Alex/Prototype_Book/Book_UI_Pawn` _returnvalue))
      (set `/Game/Alex/Prototype_Book/Book_UI_Pawn.Page` 3 _asbook_ui_pawn_3))))

(event `InputAxis|LookUp` :overrideparent false
  (params (AxisValue :type "Float (single-precision)"))
  ;[1 1 1] Mouse Movement input
  (`self.AddControllerPitchInput` AxisValue))

(event `self.ReceivePossessed`
  (params (NewController :type "Controller Object Reference"))
  ;[1 1 1] Hide or show the cross hair UI accordingly: show cross hair if the player is viewing from this first person camera.
  (`WidgetBlueprintLibrary.SetInputMode_GameOnly` (`GameplayStatics.GetPlayerController` 0))
  (`/Engine/EditorBlueprintResources/StandardMacros.IsValid` (`self.xHairWidget`)
    (:`Is Valid`
      (`UserWidget.AddToViewport` (`self.xHairWidget`) 0))
    (:`Is Not Valid`
      (`self.CreateXHairWidget`))))

(event `InputAxis|MoveRight`
  (params (AxisValue :type "Float (single-precision)"))
  ;[1 1 1] Movement Keys Input
  (bind _output_get (set `self.RightInputAxisValue` AxisValue))
  (`self.AddMovementInput` (`KismetMathLibrary.GetRightVector` (`self.GetControlRotation`)) _output_get))

(event `self.ReceiveUnpossessed`
  (params (OldController :type "Controller Object Reference"))
  ;[1 1 1] Hide or show the cross hair UI accordingly: show cross hair if the player is viewing from this first person camera.
  (`Widget.RemoveFromParent` (`self.xHairWidget`)))

(event `Key|LeftMouseButton`
  (params (Key :type "Key Structure"))
  ;[1 1 1] Mouse Clicking Input
  (:`Pressed`
    (bind (_hitactor _hitworldlocation _hitbonename _hitcomponent _ispickup_) (`self.CheckTrace`))
    ;;[1 1 1] Pickable object is hovered and clicked
    (if _ispickup_
      (if (`self.PhysicsHandleActive`)
        (set `self.PhysicsHandleActive` false)
        (`self.DropObject`)
        (else
          (set `self.PhysicsHandleActive` true)
          (`self.GrabObject`)))
      (else
        ;[1 1 1] The Clicked Actor is not a pickup
        (message `/Game/Hou/Blueprints/Interface_Interaction.OnInteracted` _hitactor)))))

(event `self.ReceiveTick`
  (params (DeltaSeconds :type "Float (single-precision)"))
  (bind _xhairwidget (`self.xHairWidget`))
  (bind _headbobamp (`self.HeadbobAmp`))
  (bind _returnvalue (* 360.0 (`self.GetNormalizedStepCycle`)))
  ;[1 1 1] Frame Updates
  (if (== (`GameplayStatics.GetPlayerPawn` 0) self)
    (`|ExecutionSequence`
      (:`then_0`
        (if (`self.PhysicsHandleActive`)
          (`self.UpdatePhysicsHandle`)
          (else
            ;[1 1 1] Not holding an object. Line trace (not happening every frame for better performance), then show the appropriate crosshair.
            (set `self.CheckTraceTimer` (+ (`self.CheckTraceTimer`) DeltaSeconds))
            (if (>= (`self.CheckTraceTimer`) (`self.CheckTraceDelay`))
              (set `self.CheckTraceTimer` 0.0)
              (`/Engine/EditorBlueprintResources/StandardMacros.IsValid` (`self.xHairWidget`)
                (:`Is Valid`
                  (bind (_hitactor _hitworldlocation _hitbonename _hitcomponent _ispickup_ _isinteractable_) (`self.CheckTrace`))
                  (if (or _ispickup_ _isinteractable_)
                    (`/Game/Hou/Widgets/CrosshairUI.ShowHandXhair` _xhairwidget)
                    (else
                      (`/Game/Hou/Widgets/CrosshairUI.ShowDotXhair` _xhairwidget)))))))))
      (:`then_1`
        ;[1 1 1] The stepping logic only executes if the character is walking
        (if (`CharacterMovementComponent.IsWalking` (`self.CharacterMovement`))
          (if (or (!= (`self.ForwardInputAxisValue`) 0.0) (!= (`self.RightInputAxisValue`) 0.0))
            (if (<= (`self.StepDelayTimer`) 0.0)
              (bind _output_get (set `self.StepCycle` (+ (`self.StepCycle`) (* (`KismetMathLibrary.VSize` (`self.GetVelocity`)) DeltaSeconds))))
              (if (>= _output_get (`self.NextStep`))
                (set `self.NextStep` (+ (`self.StepCycle`) (`self.StepInterval`)))
                (`self.PlayFootstepSfx`)
                (set `self.StepDelayTimer` (`self.StepDelay`))
                (set `self.SteppingRight?` (not (`self.SteppingRight?`)) :!label _label_2))
              (if (`self.SteppingRight?`)
                (set `self.SteppingDirection` 1)
                (else
                  (set `self.SteppingDirection` -1)))
              (`SceneComponent.K2_SetRelativeLocation` (`self.FirstPersonCamera`) (+ (`self.fpsCamOriginalRelLoc`) (`KismetMathLibrary.MakeVector` (* (`KismetMathLibrary.DegSin` (- _returnvalue 180.0)) _headbobamp) (* (`KismetMathLibrary.DegSin` (* _returnvalue (* (`self.SteppingDirection`) 0.5))) _headbobamp) (* (`KismetMathLibrary.DegCos` _returnvalue) (* _headbobamp 0.5)))) false false)
              (else
                (set `self.StepDelayTimer` (- (`self.StepDelayTimer`) DeltaSeconds))))
            (elif (> (`self.StepCycle`) 0.0)
              (set `self.StepCycle` 0.0)
              (set `self.NextStep` (+ (`self.StepCycle`) (`self.StepInterval`)))
              (goto _label_2))))))))

(event `InputAction|PauseGame`
  (params (Key :type "Key Structure"))
  (:`Released`
    (`self.PauseGame`)))

(fn `CheckTrace`
  (returns (HitActor :type "Actor Object Reference") (HitWorldLocation :type "Vector Structure") (HitBoneName :type Name) (HitComponent :type "PrimitiveComponent Object Reference") (`IsPickUp?` :type Boolean) (`IsInteractable?` :type Boolean))
  (bind _returnvalue (`GameplayStatics.GetPlayerCameraManager` 0))
  (bind _returnvalue_2 (`self.K2_GetActorLocation` _returnvalue))
  ;[1 1 1] Cast a ray to the center of the screen to detect what's infront of the player
  (bind (_outhit _returnvalue_3) (`KismetSystemLibrary.LineTraceSingle` _returnvalue_2 (+ _returnvalue_2 (* (`KismetMathLibrary.Normal` (`KismetMathLibrary.Conv_RotatorToVector` (`self.K2_GetActorRotation` _returnvalue))) (`self.InteractableDistance`))) "TraceTypeQuery1"))
  ;[1 1 1] Analyse the hit result, then return the hit detail & the object's category as booleans
  (if _returnvalue_3
    (bind (_bblockinghit _binitialoverlap _time _distance _location _impactpoint _normal _impactnormal _physmat _hitactor _hitcomponent _hitbonename) (`GameplayStatics.BreakHitResult` _outhit))
    (`/Engine/EditorBlueprintResources/StandardMacros.IsValid` _hitactor
      (:`Is Valid`
        (return _hitactor _location _hitbonename _hitcomponent (`self.ActorHasTag` _hitactor "Pickup") (`self.ActorHasTag` _hitactor "Interactable")))
      (:`Is Not Valid`
        _)))
  ;[1 1 1] ?Default output? if the line trace hit nothing/ an invalid obj
  (return null (0.0 0.0 0.0) "None" null false false))

(fn `CreateXHairWidget`
  ;[1 1 1] Create the crosshair widget and save it in a variable for later access
  (bind _returnvalue (`|CreateWidget` "/Game/Hou/Widgets/CrosshairUI.CrosshairUI_C"))
  (bind _output_get (set `self.xHairWidget` _returnvalue))
  (`UserWidget.AddToViewport` _output_get 0))

(fn `DropObject`
  (`PhysicsHandleComponent.ReleaseComponent` (`self.PhysicsHandle`))
  (`PrimitiveComponent.SetCollisionResponseToChannel` (`self.PhysicsObject`) "ECC_Pawn" "ECR_Block"))

(fn `GrabObject`
  (bind _returnvalue (`GameplayStatics.GetPlayerCameraManager` 0))
  (bind _returnvalue_2 (`self.K2_GetActorLocation` _returnvalue))
  ;[1 1 1] Trace from center of the screen in direction of the camera (Physicsbodys only)
  (bind (_outhit _returnvalue_3) (`KismetSystemLibrary.LineTraceSingleForObjects` _returnvalue_2 (+ _returnvalue_2 (* (`KismetMathLibrary.GetForwardVector` (`self.K2_GetActorRotation` _returnvalue)) (`self.InteractableDistance`))) (`self.ObjectTypes`)))
  ;[1 1 1] Adding a physics handle to the grabbing object
  (if _returnvalue_3
    (bind _returnvalue_4 (`AddComponent|NODE_AddPhysicsHandleComponent-1` :`RelativeTransform` (`self.GetTransform`)))
    (set `self.PhysicsHandle` _returnvalue_4)
    (bind (_bblockinghit _binitialoverlap _time _distance _location _impactpoint _normal _impactnormal _physmat _hitactor _hitcomponent _hitbonename) (`GameplayStatics.BreakHitResult` _outhit))
    (bind _output_get (set `self.PhysicsObject` _hitcomponent))
    ;[1 1 1] Grab the just created physics handle
    (`PhysicsHandleComponent.GrabComponentAtLocation` (`self.PhysicsHandle`) _hitcomponent _hitbonename (`PrimitiveComponent.GetCenterOfMass` _output_get _hitbonename))
    ;[1 1 1] Make sure the object doesn't collide with the Player Collider
    (`PrimitiveComponent.SetCollisionResponseToChannel` _hitcomponent "ECC_Pawn" "ECR_Ignore")))

(fn `PauseGame`
  (bind _returnvalue (`GameplayStatics.GetPlayerController` 0))
  (`GameplayStatics.SetGamePaused` true)
  (set `PlayerController.bShowMouseCursor` true _returnvalue)
  (`WidgetBlueprintLibrary.SetInputMode_GameAndUIEx` _returnvalue null)
  (`/Engine/EditorBlueprintResources/StandardMacros.IsValid` (`self.PauseMenu`)
    (:`Is Valid`
      (`UserWidget.AddToViewport` (`self.PauseMenu`) 0))
    (:`Is Not Valid`
      (bind _returnvalue_2 (`|CreateWidget` "/Game/Hou/Widgets/Widget_PauseMenu.Widget_PauseMenu_C"))
      (bind _output_get (set `self.PauseMenu` _returnvalue_2))
      (`UserWidget.AddToViewport` _output_get 0))))

(fn `PlayFootstepSfx`
  (bind _footstepsfxsequence (`self.FootstepSFXSequence`))
  ;[1 1 1] The footstep sound effect plays in sequence. Set the sequence back to zero if the current sequence exceeds the (total footstep sfx count - 1).
  (switch `int` (`self.FootstepSFXSequence`)
    (:`0`
      (`GameplayStatics.PlaySound2D` "/Game/Audio/Footsteps/heavyfootstep_sfx1.heavyfootstep_sfx1" 1.0 1.0 0.0 null null))
    (:`1`
      (`GameplayStatics.PlaySound2D` "/Game/Audio/Footsteps/heavyfootstep_sfx2.heavyfootstep_sfx2" 1.0 1.0 0.0 null null))
    (:`2`
      (`GameplayStatics.PlaySound2D` "/Game/Audio/Footsteps/heavyfootstep_sfx3.heavyfootstep_sfx3" 1.0 1.0 0.0 null null))
    (:`3`
      (`GameplayStatics.PlaySound2D` "/Game/Audio/Footsteps/heavyfootstep_sfx4.heavyfootstep_sfx4" 1.0 1.0 0.0 null null)))
  (`/Engine/EditorBlueprintResources/StandardMacros.IncrementInt` _footstepsfxsequence
    (:`  `
      (if (> _footstepsfxsequence 3)
        (set `self.FootstepSFXSequence` 0)))))

(fn `UnpauseGame`
  (bind _returnvalue (`GameplayStatics.GetPlayerController` 0))
  (`GameplayStatics.SetGamePaused` false)
  (set `PlayerController.bShowMouseCursor` false _returnvalue)
  (`WidgetBlueprintLibrary.SetInputMode_GameOnly` _returnvalue)
  (`Widget.RemoveFromParent` (`self.PauseMenu`)))

(fn `UpdatePhysicsHandle`
  ;[1 1 1] Set the physics handle to be always in front of the player
  (`PhysicsHandleComponent.SetTargetLocation` (`self.PhysicsHandle`) (+ (+ (`self.K2_GetActorLocation`) (* (`KismetMathLibrary.GetForwardVector` (`self.GetControlRotation`)) (`self.HandleDistance`))) (0.0 0.0 70.0))))

(fn `UserConstructionScript`)