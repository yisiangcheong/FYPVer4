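; Parent Blueprint for the clickable buttons on BP_PhonePuzzle, which it finds as its attach parent actor.
; While no call is active, click and release play timelines that slide the mesh along the numpad normal's up vector.
; Timeline events trigger press and dial-tone sounds, and on release numpad buttons register their Value with the puzzle.
; Interaction events and interactability checks defer to the phone puzzle.
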(event `self.ReceiveBeginPlay`
  (bind _asbp_phone_puzzle (cast `/Game/Hou/Blueprints/BP_PhonePuzzle` (`self.GetAttachParentActor`)))
  (set `self.PhonePuzzle` _asbp_phone_puzzle)
  (set `self.ButtonOriginalOffset` (`SceneComponent.RelativeLocation` (`self.PhoneButtonMesh`))))

(event `self.PhoneButtonMesh.OnClicked`
  (params (TouchedComponent :type "PrimitiveComponent Object Reference") (ButtonPressed :type "Key Structure"))
  (if (not (`/Game/Hou/Blueprints/BP_PhonePuzzle.IsPhoneOnCall?` (`self.PhonePuzzle`)))
    (bind (_direction _zoffset) (`Timeline|PressedAnim` :!via `PlayFromStart`)
      (:`Update`
        (`SceneComponent.K2_SetRelativeLocation` (`self.PhoneButtonMesh`) (+ (`self.ButtonOriginalOffset`) (* (`SceneComponent.GetUpVector` (`/Game/Hou/Blueprints/BP_PhonePuzzle.NumPad_Normal` (`self.PhonePuzzle`))) _zoffset)) false false))
      (:`PlayPressedSfx`
        (`AudioComponent.Play` (`self.PressedSfx`) 0.0)))))

(event `self.PhoneButtonMesh.OnReleased`
  (params (TouchedComponent :type "PrimitiveComponent Object Reference") (ButtonReleased :type "Key Structure"))
  (bind _dialsfx (`self.DialSfx`))
  (if (not (`/Game/Hou/Blueprints/BP_PhonePuzzle.IsPhoneOnCall?` (`self.PhonePuzzle`)))
    (`ActorComponent.SetActive` (`self.PressedAnim`) false false)
    (bind (_direction _zoffset) (`Timeline|ReleasedAnim` :!via `PlayFromStart`)
      (:`Update`
        (`SceneComponent.K2_SetRelativeLocation` (`self.PhoneButtonMesh`) (+ (`self.ButtonOriginalOffset`) (* (`SceneComponent.GetUpVector` (`/Game/Hou/Blueprints/BP_PhonePuzzle.NumPad_Normal` (`self.PhonePuzzle`))) _zoffset)) false false))
      (:`ButtonReleased`
        (`AudioComponent.Play` (`self.PressedSfx`) 0.0)
        (`AudioComponent.SetSound` _dialsfx (`self.NumpadDialTone`))
        (`AudioComponent.Play` _dialsfx 0.0)
        (if (`self.IsNumpadButton?`)
          (`/Game/Hou/Blueprints/BP_PhonePuzzle.RegisterButtonValue` (`self.PhonePuzzle`) (`self.Value`)))))))

(event `/Game/Hou/Blueprints/Interface_Interaction.OnInteracted`
  ;[1 1 1] Trigger the interacted event in phone puzzle.
  (`/Game/Hou/Blueprints/BP_PhonePuzzle.OnInteracted` (`self.PhonePuzzle`)))

(fn `CanInteract?`
  (returns (`CanBeInteracted?` :type Boolean))
  (return (`/Game/Hou/Blueprints/BP_PhonePuzzle.CanBeInteracted?` (`self.PhonePuzzle`))))

(fn `UserConstructionScript`)