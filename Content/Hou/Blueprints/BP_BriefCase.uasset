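; Briefcase combination-lock puzzle pawn that the player possesses on interaction, with a mouse cursor and mouse-over events, and leaves with Escape.
; The mouse wheel rolls the current BP_DigitPrism, chosen through SetCurrentPrism, then VerifyPassword checks the four digits against Password.
; A match opens the case, returns control, plays closing-clue audio with subtitles, closes MemoryPortal and disables interaction.
; The player pawn is notified when that audio ends; keyboard prism controls are deprecated and disconnected.
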(event `InputAxisKey|MouseWheelAxis`
  (params (AxisValue :type "Float (single-precision)"))
  (bind _subtitleactor (`self.SubtitleActor`))
  (bind _output (`|GetArrayItem` (`self.DigitPrismBPRefs`) (`self.CurrentPrismID`)))
  ;[1 1 1] Mouse Control
  (if (!= AxisValue 0.0)
    (`/Engine/EditorBlueprintResources/StandardMacros.IsValid` _output
      (:`Is Valid`
        (`/Game/Hou/Blueprints/BP_DigitPrism.AddRoll` _output (* (`KismetMathLibrary.SignOfFloat` AxisValue) (`self.MouseWheelSensitivity`)))
        ;[1 1 1] Win Condition. Win logic goes after the true pin.
        (bind _bingo_ (`self.VerifyPassword`))
        (if _bingo_
          ;[1 1 1] Play Brief Case Open Animation
          (`SkeletalMeshComponent.PlayAnimation` (`self.Briefcase_Animation_Box1561`) "/Game/Hou/3D_Placeholder/Briefcase/Briefcase_Animation_Box1561_Anim.Briefcase_Animation_Box1561_Anim" false)
          (`KismetSystemLibrary.Delay` 0.75)
          (`self.ExitBriefcasePuzzle`)
          (set `self.CanBeInteracted` false)
          (`KismetSystemLibrary.Delay` 0.5)
          ;[1 1 1] Play Closing Clues
          (`AudioComponent.Play` (`self.ClosingClues`) 0.0)
          (`PrimitiveComponent.SetCollisionEnabled` (`self.Briefcase_Animation_Box1561`) "NoCollision")
          (`PrimitiveComponent.SetCollisionEnabled` (`self.Briefcase_Animation_Box1560`) "NoCollision")
          (`PrimitiveComponent.SetCollisionEnabled` (`self.Briefcase_Animation_Box1558`) "NoCollision")
          (`/Game/Siang/ItemClass/MemoryContainer_BP.Close` (`self.MemoryPortal`))
          (for _array_element (`self.DigitPrismBPRefs`)
            (`SceneComponent.SetHiddenInGame` (`/Game/Hou/Blueprints/BP_DigitPrism.Code_Block` _array_element) true false))
          (`self.SetActorEnableCollision` false)
          (`/Game/Siang/Dialogue/Subtitle_BP.DialogueEnable` _subtitleactor self 2 (`/Game/Siang/Dialogue/Subtitle_BP.SubInterval` _subtitleactor))
          (`PrimitiveComponent.SetCollisionEnabled` (`/Game/Siang/Dialogue/Subtitle_BP.Box` _subtitleactor) "NoCollision"))))))

(event `/Game/Hou/Blueprints/Interface_Interaction.OnInteracted`
  (bind _returnvalue (`GameplayStatics.GetPlayerController` 0))
  ;[1 1 1] React when the player points and clicked on the briefcase.
  (if (`self.CanBeInteracted`)
    (set `self.PlayerPawnReference` (`Controller.K2_GetPawn` (`GameplayStatics.GetPlayerController` 0)))
    (`Controller.Possess` _returnvalue self)
    (set `PlayerController.bShowMouseCursor` true _returnvalue)
    (`WidgetBlueprintLibrary.SetInputMode_GameAndUIEx` _returnvalue null "DoNotLock" false)
    (set `PlayerController.bEnableMouseOverEvents` true _returnvalue)))

(event `Key|W`
  (params (Key :type "Key Structure"))
  ;[1 1 1] WASD Input Handling (Deprecated)
)

(event `Key|Escape`
  (params (Key :type "Key Structure"))
  ;[1 1 1] Exit the brief case puzzle
  (:`Released`
    (`self.ExitBriefcasePuzzle`)))

(event `Key|S`
  (params (Key :type "Key Structure"))
  ;[1 1 1] WASD Input Handling (Deprecated)
)

(event `Key|D`
  (params (Key :type "Key Structure"))
  ;[1 1 1] WASD Input Handling (Deprecated)
)

(event `Key|A`
  (params (Key :type "Key Structure"))
  ;[1 1 1] WASD Input Handling (Deprecated)
)

(event `self.ClosingClues.OnAudioFinished`
  ;[1 1 1] Briefcase closing clues has ended, notify the player.
  (message `/Game/Hou/Blueprints/Interface_PuzzleUpdate.OnClosingClueEnded` (`self.PlayerPawnReference`) "NewEnumerator2"))

(fn `ExitBriefcasePuzzle`
  (bind _returnvalue (`GameplayStatics.GetPlayerController` 0))
  (`Controller.Possess` _returnvalue (`self.PlayerPawnReference`))
  (set `PlayerController.bShowMouseCursor` false _returnvalue)
  (`WidgetBlueprintLibrary.SetInputMode_GameOnly` _returnvalue)
  (set `PlayerController.bEnableMouseOverEvents` false _returnvalue))

(fn `SetCurrentPrism`
  (params (CurrentPrismID :type Integer))
  (set `self.CurrentPrismID` CurrentPrismID))

(fn `UpdatePrismID (Deprecated)`
  (params (`Value To Add` :type Integer))
  (locals (InitialID :type Integer))
  (bind _currentprismid (`self.CurrentPrismID`))
  (set `local.InitialID` _currentprismid)
  (set `self.CurrentPrismID` (+ _currentprismid `Value To Add`))
  (if (> (`self.CurrentPrismID`) 3)
    (set `self.CurrentPrismID` 0)
    (elif (< (`self.CurrentPrismID`) 0)
      (set `self.CurrentPrismID` 3))))

(fn `UserConstructionScript`)

(fn `VerifyPassword`
  (returns (`Bingo?` :type Boolean))
  (locals (Local_PasswordInput :type Integer) (Local_DigitValue :type Integer))
  (for (_array_element _array_index) (`self.DigitPrismBPRefs`)
    (switch `int` _array_index
      (:`0`
        (set `local.Local_DigitValue` 1000))
      (:`1`
        (set `local.Local_DigitValue` 100))
      (:`2`
        (set `local.Local_DigitValue` 10))
      (:`3`
        (set `local.Local_DigitValue` 1)))
    (set `local.Local_PasswordInput` (+ (`local.Local_PasswordInput`) (* (`/Game/Hou/Blueprints/BP_DigitPrism.Value` _array_element) (`local.Local_DigitValue`)))))
  (return (== (`local.Local_PasswordInput`) (`self.Password`))))