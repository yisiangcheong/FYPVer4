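; Parent Blueprint for a note puzzle piece that scatters with random position and yaw on BeginPlay and routes clicks and interaction to its NotePuzzle.
; With RefreshNeighborData set, the construction script bakes each neighbor's distance and look-at yaw from the placed layout.
; SnapWithNeighbor tests orientation, distance and angle within tolerances against neighbors outside its container.
; A match moves the piece, or its container root, into place and restores both original rotations.
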(event `self.ReceiveBeginPlay`
  (set `self.OringialRotation` (`self.K2_GetActorRotation`))
  (`self.K2_AddActorWorldRotation` (`KismetMathLibrary.MakeRotator` 0.0 0.0 (* (`KismetMathLibrary.RandomInteger` 72) 5.0)))
  ;[1 1 1] Reset this piece's position to the puzzle's origin
  (`self.K2_SetActorRelativeLocation` (`KismetMathLibrary.RandomPointInBoundingBox` (0.0 0.0 0.0) (9.0 0.0 6.25))))

(event `/Game/Hou/Blueprints/Interface_Interaction.OnInteracted`
  ;[1 1 1] Redirect to interact with the note puzzle
  (`/Game/Hou/Blueprints/BP_NotePuzzle.OnInteracted` (`self.Note Puzzle`)))

(event `self.BoxCollider.OnClicked`
  (params (TouchedComponent :type "PrimitiveComponent Object Reference") (ButtonPressed :type "Key Structure"))
  (bind _note_puzzle (`self.Note Puzzle`))
  (`/Engine/EditorBlueprintResources/StandardMacros.IsValid` _note_puzzle
    (:`Is Valid`
      (`/Game/Hou/Blueprints/BP_NotePuzzle.GrabPiece` _note_puzzle self))))

(event `self.Mesh.OnClicked`
  (params (TouchedComponent :type "PrimitiveComponent Object Reference") (ButtonPressed :type "Key Structure"))
  (bind _note_puzzle (`self.Note Puzzle`))
  (`/Engine/EditorBlueprintResources/StandardMacros.IsValid` _note_puzzle
    (:`Is Valid`
      (`/Game/Hou/Blueprints/BP_NotePuzzle.GrabPiece` _note_puzzle self))))

(fn `GetInteractionStatus`
  (returns (`Interaction Status` :type "/Game/Hou/Blueprints/Enum_InteractionStatus Enum"))
  (if (`/Game/Hou/Blueprints/BP_NotePuzzle.FirstInteract` (`self.Note Puzzle`))
    (if (`/Game/Hou/Blueprints/BP_NotePuzzle.CanBeInteracted?` (`self.Note Puzzle`))
      (return "NewEnumerator1")
      (else
        (return "NewEnumerator0")))
    (else
      (return "NewEnumerator2"))))

(fn `HasCorrectRotation?`
  (returns (True :type Boolean))
  (return (> (`KismetMathLibrary.Dot_VectorVector` (`KismetMathLibrary.Conv_RotatorToVector` (`self.K2_GetActorRotation`)) (`KismetMathLibrary.Conv_RotatorToVector` (`self.OringialRotation`))) 0.96)))

(fn `SnapWithNeighbor`
  (params (DistDeviation :type "Float (double-precision)") (AngleDeviation :type "Float (double-precision)"))
  (returns (Success :type Boolean) (CurrentPiece :type "/Game/Hou/Blueprints/BP_NotePieces/BP_NotePiece_Parent Object Reference") (Neighbor :type "/Game/Hou/Blueprints/BP_NotePieces/BP_NotePiece_Parent Object Reference"))
  (locals (Local_DistDeviation :type "Float (double-precision)") (Local_AngleDeviation :type "Float (double-precision)") (Local_DesiredPosition :type "Vector Structure") (Local_NeighborPieceRef :type "/Game/Hou/Blueprints/BP_NotePieces/BP_NotePiece_Parent Object Reference"))
  (bind _local_distdeviation (`local.Local_DistDeviation`))
  (bind _local_angledeviation (`local.Local_AngleDeviation`))
  (bind _container_root (break `/Game/Hou/Blueprints/Struct_PieceContainer` (`self.Container`)))
  (bind _local_neighborpieceref (`local.Local_NeighborPieceRef`))
  (bind (_container_root_2 _container_notepiecechildren) (break `/Game/Hou/Blueprints/Struct_PieceContainer` (`self.Container`)))
  (bind (_returnvalue_x _returnvalue_y _returnvalue_z) (`KismetMathLibrary.BreakVector` (`SceneComponent.K2_GetComponentLocation` (`self.RootComponent`))))
  (bind (_returnvalue_x_2 _returnvalue_y_2) (`KismetMathLibrary.BreakVector` (`SceneComponent.K2_GetComponentLocation` (`Actor.RootComponent` (`local.Local_NeighborPieceRef`)))))
  (bind _returnvalue (`KismetMathLibrary.VSize` (- (`SceneComponent.K2_GetComponentLocation` (`self.RootComponent`)) (`SceneComponent.K2_GetComponentLocation` (`Actor.RootComponent` (`local.Local_NeighborPieceRef`))))))
  (bind _yaw (.yaw (`KismetMathLibrary.FindLookAtRotation` (`SceneComponent.K2_GetComponentLocation` (`self.RootComponent`)) (`SceneComponent.K2_GetComponentLocation` (`Actor.RootComponent` (`local.Local_NeighborPieceRef`))))))
  (set `local.Local_AngleDeviation` AngleDeviation)
  (set `local.Local_DistDeviation` DistDeviation)
  (for _array_element (`self.NeighborData`)
    (bind (_neighborpieceref _matchingdist _matchingangleto) (break `/Game/Hou/Blueprints/Struct_PieceNeighbor` _array_element))
    (set `local.Local_NeighborPieceRef` _neighborpieceref)
    ;[1 1 1] Avoid (re)snapping to a snapped piece
    (if (not (`KismetArrayLibrary.Array_Contains` _container_notepiecechildren (`local.Local_NeighborPieceRef`)))
      (bind _true (`self.HasCorrectRotation?`))
      (if _true
        (bind _true_2 (`self.HasCorrectRotation?` (`local.Local_NeighborPieceRef`)))
        (if _true_2
          (if (and (> _returnvalue (- _matchingdist _local_distdeviation)) (< _returnvalue (+ _matchingdist _local_distdeviation)))
            (if (and (> _yaw (- _matchingangleto _local_angledeviation)) (< _yaw (+ _matchingangleto _local_angledeviation)))
              (bind _returnvalue_2 (+ _matchingangleto 180.0))
              (set `local.Local_DesiredPosition` (`KismetMathLibrary.MakeVector` (+ (* (`KismetMathLibrary.DegCos` _returnvalue_2) _matchingdist) _returnvalue_x_2) (+ _returnvalue_y_2 (* _matchingdist (`KismetMathLibrary.DegSin` _returnvalue_2))) _returnvalue_z))
              (`/Engine/EditorBlueprintResources/StandardMacros.IsValid` _container_root
                (:`Is Valid`
                  (`self.K2_AddActorWorldOffset` _container_root (- (`local.Local_DesiredPosition`) (`SceneComponent.K2_GetComponentLocation` (`self.RootComponent`))) false false))
                (:`Is Not Valid`
                  (`SceneComponent.K2_SetWorldLocation` (`self.RootComponent`) (`local.Local_DesiredPosition`) false false)))
              (`self.K2_SetActorRotation` (`self.OringialRotation`))
              (`self.K2_SetActorRotation` _local_neighborpieceref (`/Game/Hou/Blueprints/BP_NotePieces/BP_NotePiece_Parent.OringialRotation` _local_neighborpieceref) false)
              (return true self (`local.Local_NeighborPieceRef`))))))))
  (return false null null))

(fn `UserConstructionScript`
  (bind _returnvalue (`SceneComponent.K2_GetComponentLocation` (`self.RootComponent`)))
  (if (`self.RefreshNeighborData`)
    (for (_array_element _array_index) (`self.NeighborData`)
      (bind _returnvalue_2 (`SceneComponent.K2_GetComponentLocation` (`Actor.RootComponent` (`.NeighborPieceRef_10_F1184CE74077908663DD24AD8E29BEDE` (break `/Game/Hou/Blueprints/Struct_PieceNeighbor` _array_element)))))
      (bind _structout (setmembers `/Game/Hou/Blueprints/Struct_PieceNeighbor` :`StructRef` _array_element :`MatchingDist` (`KismetMathLibrary.VSize` (- _returnvalue _returnvalue_2))))
      (bind _structout_2 (setmembers `/Game/Hou/Blueprints/Struct_PieceNeighbor` :`StructRef` _structout :`MatchingAngleTo` (.yaw (`KismetMathLibrary.FindLookAtRotation` _returnvalue _returnvalue_2))))
      (`KismetArrayLibrary.Array_Set` (`self.NeighborData`) _array_index _structout_2))))