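; Possessable phone puzzle where the player dials a series of numbers in order, hearing subtitled conversations until the last closes the memory portal.
; Interaction possesses the phone and lerps the camera in; buttons build a number checked against the current entry, with easter-egg and not-in-service fallbacks.
; Finished calls swap the number note and lower LUT intensity.
; The fourth call runs an extension-menu state machine, with Tick replaying idle prompts.
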(event `Easter Egg Call`
  (bind _audio (`self.Audio`))
  (bind _audio_2 (`self.Audio`))
  (bind _subtitleactor (`self.SubtitleActor`))
  (`AudioComponent.SetSound` _audio "/Game/Audio/sfx_internal_phone_ring.sfx_internal_phone_ring")
  (`AudioComponent.Play` _audio 1.7) ; Play dialing sfx (one ring)
  (`KismetSystemLibrary.Delay` 1.7)
  (`AudioComponent.SetSound` _audio_2 "/Game/Sounds/Puzzle/Phone/easter_egg.easter_egg")
  (`AudioComponent.Play` _audio_2 0.0)
  (`/Game/Siang/Dialogue/Subtitle_BP.DialogueEnable` _subtitleactor self 10 0.0 false null 0)
  (set `/Game/Siang/Dialogue/Subtitle_BP.SubArrayInt` 33 _subtitleactor))

(event `self.ReceiveBeginPlay`
  (set `self.CameraOriPos` (`SceneComponent.K2_GetComponentToWorld` (`self.Camera`)))
  (`self.ClearInputValue`))

(event `Picked Up Call`
  (params (`Dialing Delay` :type "Float (double-precision)"))
  (bind _audio (`self.Audio`))
  (bind _subtitleactor (`self.SubtitleActor`))
  (bind (_output_phonenumber _output_audiocue _output_conversationid _output_subintervalint) (break `/Game/Hou/Blueprints/Struct_NumberToCall` (`|GetArrayItem` (`self.PhoneNumbersToCall`) (`self.PhoneNumberCalled`))))
  (`self.DialogueTerminate`)
  (set `self.IsPhoneOnCall?` true)
  (`MovieSceneSequencePlayer.Play` (`LevelSequenceActor.SequencePlayer` (`self.FadesOutSequence`)))
  (`KismetSystemLibrary.Delay` `Dialing Delay`) ; Mainly delay for the Doo Doo Sound
  (`AudioComponent.SetSound` _audio _output_audiocue)
  (`AudioComponent.Play` _audio 0.0)
  (set `/Game/Siang/Dialogue/Subtitle_BP.SubArrayInt` _output_subintervalint _subtitleactor)
  (`/Game/Siang/Dialogue/Subtitle_BP.DialogueEnable` _subtitleactor self _output_conversationid 0.0 false null 0))

(event `Not in Service Call`
  (bind _audio (`self.Audio`))
  (bind _audio_2 (`self.Audio`))
  (`AudioComponent.SetSound` _audio "/Game/Audio/sfx_internal_phone_ring.sfx_internal_phone_ring")
  (`AudioComponent.Play` _audio 1.7) ; Play dialing sfx (one ring)
  (`KismetSystemLibrary.Delay` 1.7)
  (`AudioComponent.SetSound` _audio_2 "/Game/Sounds/Puzzle/Phone/Telephone_Announcer_2.Telephone_Announcer_2")
  (`AudioComponent.Play` _audio_2 0.0) ; Not in service audio
)

(event `/Game/Hou/Blueprints/Interface_Interaction.OnInteracted`
  (bind _returnvalue (`GameplayStatics.GetPlayerController` 0))
  (bind _audio (`self.Audio`))
  (if (`self.FirstInteract`)
    ;[1 1 1] React when the player points and clicked on the phone.
    (if (`self.CanBeInteracted?`)
      (set `self.PlayerCamOriPos` (`SceneComponent.K2_GetComponentToWorld` (`PlayerCameraManager.TransformComponent` (`GameplayStatics.GetPlayerCameraManager` 0))))
      (set `self.PlayerPawnReference` (`Controller.K2_GetPawn` (`GameplayStatics.GetPlayerController` 0)))
      (`Controller.Possess` _returnvalue self)
      ;[1 1 1] Alex's book disabled
      (bind _asnew_player_controller (cast `/Game/Alex/NewPlayerController` (`GameplayStatics.GetPlayerController` 0)))
      (set `/Game/Alex/NewPlayerController.InPuzzle` true _asnew_player_controller)
      ;[1 1 1] Camera Lerp
      (bind (_direction _lerpfloat) (`Timeline|CameraLerpIntoPuzzle` :!via `PlayFromStart`)
        (:`Update`
          (`SceneComponent.K2_SetWorldTransform` (`self.Camera`) (`KismetMathLibrary.TLerp` (`SceneComponent.K2_GetComponentToWorld` (`PlayerCameraManager.TransformComponent` (`GameplayStatics.GetPlayerCameraManager` 0))) (`self.CameraOriPos`) _lerpfloat) false false))
        (:`Finished`
          (set `PlayerController.bShowMouseCursor` true _returnvalue)
          (set `PlayerController.bEnableMouseOverEvents` true _returnvalue)
          (`WidgetBlueprintLibrary.SetInputMode_GameAndUIEx` _returnvalue null)
          (`PrimitiveComponent.SetCollisionEnabled` (`self.phone_lp_phone_body`) "NoCollision") ; Prevent the phone body's collider from blocking the buttons.
          ;[1 1 1] Start the dial tone
          (if (not (`self.IsPhoneOnCall?`))
            (`AudioComponent.SetSound` _audio "/Game/Sounds/Puzzle/Phone/Dial_Tone.Dial_Tone")
            (`AudioComponent.Play` _audio 0.0)))))
    (else
      (set `self.FirstInteract` true)
      (`/Game/Siang/ItemClass/MemoryContainer_BP.FirstInteract` (`self.MemoryPortal`))
      (`self.SetActorEnableCollision` (`self.SubtitleActor`) true))))

(event `/Game/Hou/Blueprints/Interface_PuzzleUpdate.OnDialogueFinished`
  (bind _audio (`self.Audio`))
  (bind _postprocess (`/Game/Siang/ItemClass/MemoryContainer_BP.PostProcess` (`self.MemoryPortal`)))
  (bind _postprocess_2 (`/Game/Siang/ItemClass/MemoryContainer_BP.PostProcess` (`self.MemoryPortal`)))
  (bind _postprocess_3 (`/Game/Siang/ItemClass/MemoryContainer_BP.PostProcess` (`self.MemoryPortal`)))
  (if (`self.IsPhoneOnCall?`)
    (set `self.IsPhoneOnCall?` false)
    (if (`self.IsBeingPossessed?`)
      (`MovieSceneSequencePlayer.Play` (`LevelSequenceActor.SequencePlayer` (`self.FadesInSequence`)))
      (`AudioComponent.SetSound` _audio "/Game/Sounds/Puzzle/Phone/Dial_Tone.Dial_Tone") ; Play the dial tone again
      (`AudioComponent.Play` _audio 0.0))
    (bind _result (`/Engine/EditorBlueprintResources/StandardMacros.IncrementInt` (`self.PhoneNumberCalled`)) ; Dialed 1 phone number
      (:`  `
        (switch `int` _result
          (:`Default`
            _)
          (:`1`
            (bind _structout (setmembers `PostProcessSettings` :`StructRef` (`PostProcessComponent.Settings` _postprocess_2) :`ColorGradingIntensity` 0.666666))
            (set `PostProcessComponent.Settings` _structout _postprocess_2)
            (`SceneComponent.SetVisibility` (`self.PNum_P1`) false true)
            (`SceneComponent.SetVisibility` (`self.PNum_P2`) true true))
          (:`2`
            (bind _structout_2 (setmembers `PostProcessSettings` :`StructRef` (`PostProcessComponent.Settings` _postprocess_3) :`ColorGradingIntensity` 0.333333))
            (set `PostProcessComponent.Settings` _structout_2 _postprocess_3)
            (`SceneComponent.SetVisibility` (`self.PNum_P2`) false true)
            (`SceneComponent.SetVisibility` (`self.PNum_P3`) true true))
          (:`3`
            (bind _structout_3 (setmembers `PostProcessSettings` :`StructRef` (`PostProcessComponent.Settings` _postprocess) :`ColorGradingIntensity` 0.0))
            (set `PostProcessComponent.Settings` _structout_3 _postprocess)
            (`SceneComponent.SetVisibility` (`self.PNum_P3`) false true)
            (`SceneComponent.SetVisibility` (`self.PNum_P4`) true true)))
        (if (>= (`self.PhoneNumberCalled`) (`KismetArrayLibrary.Array_Length` (`self.PhoneNumbersToCall`)))
          (set `self.Win?` true))
        ;[1 1 1] All the phone number has been dialed and the conversation has ended. Puzzle solved. Win logic goes after this.
        (if (`self.Win?`)
          ;[1 1 1] Camera Lerp Reverse
          (bind (_direction _lerpfloat) (`Timeline|Timeline_1` :!via `ReverseFromEnd`)
            (:`Update`
              (`SceneComponent.K2_SetWorldTransform` (`self.Camera`) (`KismetMathLibrary.TLerp` (`self.PlayerCamOriPos`) (`self.CameraOriPos`) _lerpfloat) false false))
            (:`Finished`
              (`self.ExitPuzzle`)
              (`ActorComponent.Deactivate` (`Emitter.ParticleSystemComponent` (`self.ParticleEmitter`)))
              (set `self.CanBeInteracted?` false)
              (`/Game/Siang/ItemClass/MemoryContainer_BP.Close` (`self.MemoryPortal`))
              (message `/Game/Hou/Blueprints/Interface_PuzzleUpdate.OnClosingClueEnded` (`self.PlayerPawnReference`) "NewEnumerator7")
              (`PrimitiveComponent.SetCollisionEnabled` (`/Game/Siang/Dialogue/Subtitle_BP.Box` (`self.SubtitleActor`)) "NoCollision")
              (set `/Game/Siang/Dialogue/Subtitle_BP.FinishedPuzzle` true (`self.SubtitleActor`)))))))))

(event `Key|Escape`
  (params (Key :type "Key Structure"))
  ;[1 1 1] Exit the phone puzzle
  (:`Released`
    (if (not (`self.IsPhoneOnCall?`))
      ;[1 1 1] Camera Lerp Reverse
      (bind (_direction _lerpfloat) (`Timeline|Timeline_2` :!via `ReverseFromEnd`)
        (:`Update`
          (`SceneComponent.K2_SetWorldTransform` (`self.Camera`) (`KismetMathLibrary.TLerp` (`self.PlayerCamOriPos`) (`self.CameraOriPos`) _lerpfloat) false false))
        (:`Finished`
          (`self.ExitPuzzle`))))))

(event `Phone Call`
  (bind _audio (`self.Audio`))
  (bind _audio_2 (`self.Audio`))
  (if (not (== (`self.PhoneNumberCalled`) 3))
    (`AudioComponent.SetSound` _audio_2 "/Game/Audio/sfx_internal_phone_ring.sfx_internal_phone_ring")
    (`AudioComponent.Play` _audio_2 0.0) ; Play dialing sfx (two ring)
    (`self.Picked Up Call` 3.4) ; Delay 3.4s for the sfx
    (else
      (`AudioComponent.SetSound` _audio "/Game/Audio/sfx_internal_phone_ring.sfx_internal_phone_ring")
      (`AudioComponent.Play` _audio 1.7) ; Play dialing sfx (one ring)
      (`KismetSystemLibrary.Delay` 1.7)
      (`self.ChangeExtSequence` 1)
      (`self.ProcessExtensionSeq`))))

(event `self.ReceiveTick`
  (params (DeltaSeconds :type "Float (single-precision)"))
  (bind _subtitleactor (`self.SubtitleActor`))
  (if (`self.IsBeingPossessed?`)
    (if (and (and (not (`self.IsPhoneOnCall?`)) (`self.IsOnCallWithExtension?`)) (not (`AudioComponent.IsPlaying` (`self.Audio`))))
      (bind _output_get (set `self.ExtTimeElapsed` (+ (`self.ExtTimeElapsed`) DeltaSeconds)))
      (if (>= _output_get 5.0)
        (`AudioComponent.Play` (`self.Audio`) 0.0) ; Replay the sound set previously
        (`/Game/Siang/Dialogue/Subtitle_BP.DialogueEnable` _subtitleactor self (`/Game/Siang/Dialogue/Subtitle_BP.Conversation_ID` _subtitleactor) 0.0 false null 0)
        (set `/Game/Siang/Dialogue/Subtitle_BP.SubArrayInt` (`self.CachedSubArrayInt`) _subtitleactor)
        (set `self.ExtTimeElapsed` 0.0) ; Reset
      ))))

(event `self.ReceiveUnpossessed`
  (params (OldController :type "Controller Object Reference"))
  (bind _cameralerpintopuzzle (`self.CameraLerpIntoPuzzle`))
  (`self.ClearInputValue`)
  (`PrimitiveComponent.SetCollisionEnabled` (`self.phone_lp_phone_body`) "QueryAndPhysics")
  ;[1 1 1] To exit from ordinary calls
  (if (`self.IsPhoneOnCall?`)
    (`MovieSceneSequencePlayer.Play` (`LevelSequenceActor.SequencePlayer` (`self.FadesInSequence`)))
    (else
      (`AudioComponent.FadeOut` (`self.Audio`) 1.0 0.0)
      (if (`self.IsOnCallWithExtension?`)
        (`self.ChangeExtSequence` -1) ; To exit from an extension call
        (`self.DialogueTerminate`))))
  (if (`TimelineComponent.IsPlaying` _cameralerpintopuzzle)
    (`TimelineComponent.Stop` _cameralerpintopuzzle)))

(event `self.Audio.OnAudioFinished`
  (bind _subtitleactor (`self.SubtitleActor`))
  (bind _subtitleactor_2 (`self.SubtitleActor`))
  (bind _audio (`self.Audio`))
  (bind _audio_2 (`self.Audio`))
  (if (== (`AudioComponent.Sound` (`self.Audio`)) "/Game/Sounds/Puzzle/Phone/ext_representative_unreached.ext_representative_unreached")
    (`KismetSystemLibrary.Delay` 0.4)
    (`AudioComponent.SetSound` _audio_2 "/Game/Sounds/Puzzle/Phone/ext_thankyouforcalling.ext_thankyouforcalling")
    (`AudioComponent.Play` _audio_2 0.0)
    (`self.ChangeExtSequence` 2)
    (`/Game/Siang/Dialogue/Subtitle_BP.DialogueEnable` _subtitleactor self 9 0.0 false null 0)
    (bind _output_get (set `/Game/Siang/Dialogue/Subtitle_BP.SubArrayInt` 29 _subtitleactor))
    (set `self.CachedSubArrayInt` _output_get)
    (elif (== (`AudioComponent.Sound` (`self.Audio`)) "/Game/Sounds/Puzzle/Phone/ext_line_unavailable.ext_line_unavailable")
      (`KismetSystemLibrary.Delay` 0.4)
      (`AudioComponent.SetSound` _audio "/Game/Sounds/Puzzle/Phone/ext_department_select.ext_department_select")
      (`AudioComponent.Play` _audio 0.0)
      (`self.ChangeExtSequence` 3)
      (`/Game/Siang/Dialogue/Subtitle_BP.DialogueEnable` _subtitleactor_2 self 7 0.0 false null 0)
      (bind _output_get_2 (set `/Game/Siang/Dialogue/Subtitle_BP.SubArrayInt` 24 _subtitleactor_2))
      (set `self.CachedSubArrayInt` _output_get_2))))

(event `DialogueTerminate`
  (bind _subtitleactor (`self.SubtitleActor`))
  (bind _dialoguewidget (`/Game/Siang/Dialogue/Subtitle_BP.DialogueWidget` (`self.SubtitleActor`)))
  (if (`/Game/Siang/Dialogue/Subtitle_BP.PreventSubDuplicate` (`self.SubtitleActor`))
    (set `/Game/Siang/Dialogue/Subtitle_BP.PreventSubDuplicate` false (`self.SubtitleActor`))
    (`/Game/Siang/Dialogue/DialogueWidget.SlideOutAnim` _dialoguewidget)
    (`KismetSystemLibrary.Delay` 0.5)
    (`Widget.RemoveFromParent` _dialoguewidget)
    (set `/Game/Siang/Dialogue/Subtitle_BP.DialogueWidget` null (`self.SubtitleActor`))
    (set `/Game/Siang/Dialogue/Subtitle_BP.LineCurrent` 0 _subtitleactor)
    (set `/Game/Siang/Dialogue/Subtitle_BP.SubtitlesOn` false _subtitleactor)
    (set `/Game/Siang/Dialogue/Subtitle_BP.PreventSubDuplicate` true _subtitleactor)
    (`/Game/Siang/Dialogue/Subtitle_BP.AudioFadeOut` _subtitleactor)))

(fn `CallNumber`
  (locals (Local_NumberIsValid :type Boolean))
  (bind _audio (`self.Audio`))
  (bind _output_phonenumber (break `/Game/Hou/Blueprints/Struct_NumberToCall` (`|GetArrayItem` (`self.PhoneNumbersToCall`) (`self.PhoneNumberCalled`))))
  ;[1 1 1] Is there any input? If it's in a call with extension, call button will hang up the phone.
  (if (and (> (`KismetStringLibrary.Len` (`self.InputValue`)) 0) (not (`self.IsOnCallWithExtension?`)))
    (if (`KismetStringLibrary.EqualEqual_StrStr` (`self.InputValue`) "+999")
      (`self.DialogueTerminate`)
      (`self.Easter Egg Call`)
      (else
        (for _array_element _output_phonenumber
          (if (`KismetStringLibrary.EqualEqual_StrStr` (`self.InputValue`) _array_element)
            (set `local.Local_NumberIsValid` true)
            (`self.Phone Call`)
            (break)))
        ;[1 1 1] The phone number called in not pre-defined
        (if (not (`local.Local_NumberIsValid`))
          (`self.DialogueTerminate`)
          (`self.Not in Service Call`))))
    (else
      ;[1 1 1] "Hang up the phone"
      (`self.ClearInputValue`)
      (`self.ChangeExtSequence` -1) ; "Exit" extension sequence, -1 represents inactive
      (`AudioComponent.SetSound` _audio "/Game/Sounds/Puzzle/Phone/Dial_Tone.Dial_Tone")
      (`AudioComponent.FadeIn` _audio 6.0 1.0 0.0)
      (`self.DialogueTerminate`))))

(fn `ChangeExtSequence`
  (params (NewSequenceNo :type Integer))
  (set `self.ExtSequenceNo` NewSequenceNo)
  (set `self.ExtTimeElapsed` 0.0) ; Reset the wait time
)

(fn `ClearInputValue`
  (bind _output_get (set `self.InputValue` ""))
  (`TextRenderComponent.K2_SetText` (`self.TextRender`) (`KismetTextLibrary.Conv_StringToText` _output_get)))

(fn `ExitPuzzle`
  (bind _returnvalue (`GameplayStatics.GetPlayerController` 0))
  (`Controller.Possess` _returnvalue (`self.PlayerPawnReference`))
  (set `PlayerController.bShowMouseCursor` false _returnvalue)
  ;[1 1 1] Necessary for the viewport to stay focused after mouse cursor is hidden
  (`WidgetBlueprintLibrary.SetInputMode_GameOnly` _returnvalue))

(fn `GetInteractionStatus`
  (returns (`Interaction Status` :type "/Game/Hou/Blueprints/Enum_InteractionStatus Enum"))
  (if (`self.FirstInteract`)
    (if (`self.CanBeInteracted?`)
      (return "NewEnumerator1")
      (else
        (return "NewEnumerator0")))
    (else
      (return "NewEnumerator2"))))

(fn `ProcessExtensionSeq`
  (bind _subtitleactor (`self.SubtitleActor`))
  (bind _subtitleactor_2 (`self.SubtitleActor`))
  (bind _subtitleactor_3 (`self.SubtitleActor`))
  (bind _audio (`self.Audio`))
  (bind _audio_2 (`self.Audio`))
  (bind _audio_3 (`self.Audio`))
  (bind _audio_4 (`self.Audio`))
  (bind _subtitleactor_4 (`self.SubtitleActor`))
  (switch `int` (`self.ExtSequenceNo`)
    (:`1`
      (`AudioComponent.SetSound` _audio_2 "/Game/Sounds/Puzzle/Phone/ext_thankyouforcalling.ext_thankyouforcalling")
      (`AudioComponent.Play` _audio_2 0.0)
      (`self.ChangeExtSequence` 2)
      (`/Game/Siang/Dialogue/Subtitle_BP.DialogueEnable` _subtitleactor self 9 0.0 false null 0)
      (bind _output_get (set `/Game/Siang/Dialogue/Subtitle_BP.SubArrayInt` 29 _subtitleactor))
      (set `self.CachedSubArrayInt` _output_get))
    (:`2`
      (switch `string` (`self.GetLatestCharInput`)
        (:`1`
          (`AudioComponent.SetSound` _audio_3 "/Game/Sounds/Puzzle/Phone/ext_representative_unreached.ext_representative_unreached" :!label _label)
          (`AudioComponent.Play` _audio_3 0.0)
          (`self.ChangeExtSequence` 2) ; Remain unchanged..
          (`/Game/Siang/Dialogue/Subtitle_BP.DialogueEnable` _subtitleactor_2 self 6 0.0 false null 0)
          (bind _output_get_2 (set `/Game/Siang/Dialogue/Subtitle_BP.SubArrayInt` 23 _subtitleactor_2))
          (set `self.CachedSubArrayInt` _output_get_2))
        (:`2`
          (goto _label))
        (:`3`
          (`AudioComponent.SetSound` _audio_4 "/Game/Sounds/Puzzle/Phone/ext_department_select.ext_department_select")
          (`AudioComponent.Play` _audio_4 0.0)
          (`self.ChangeExtSequence` 3)
          (`/Game/Siang/Dialogue/Subtitle_BP.DialogueEnable` _subtitleactor_3 self 7 0.0 false null 0)
          (bind _output_get_3 (set `/Game/Siang/Dialogue/Subtitle_BP.SubArrayInt` 24 _subtitleactor_3))
          (set `self.CachedSubArrayInt` _output_get_3))))
    (:`3`
      (switch `string` (`self.GetLatestCharInput`)
        (:`1`
          (`AudioComponent.SetSound` _audio "/Game/Sounds/Puzzle/Phone/ext_line_unavailable.ext_line_unavailable" :!label _label_2)
          (`AudioComponent.Play` _audio 0.0)
          (`self.ChangeExtSequence` 3) ; Remain unchanged..
          (`/Game/Siang/Dialogue/Subtitle_BP.DialogueEnable` _subtitleactor_4 self 8 0.0 false null 0)
          (bind _output_get_4 (set `/Game/Siang/Dialogue/Subtitle_BP.SubArrayInt` 28 _subtitleactor_4))
          (set `self.CachedSubArrayInt` _output_get_4))
        (:`2`
          (`self.ChangeExtSequence` 4) ; Switch to the next sequence which handles the final call
          (`self.ProcessExtensionSeq`))
        (:`3`
          (goto _label_2))
        (:`4`
          (goto _label_2))))
    (:`4`
      (`self.ClearInputValue`)
      (`self.Picked Up Call` 2.0))))

(fn `RegisterButtonValue`
  (params (Value :type String))
  (bind _audio (`self.Audio`))
  (if (< (`KismetStringLibrary.Len` (`self.InputValue`)) 12)
    (`|ExecutionSequence`
      (:`then_0`
        (if (== (`KismetStringLibrary.Len` (`self.InputValue`)) 0)
          (set `self.InputValue` (`KismetStringLibrary.Concat_StrStr` (`self.InputValue`) "+"))))
      (:`then_1`
        (bind _output_get (set `self.InputValue` (`KismetStringLibrary.Concat_StrStr` (`self.InputValue`) Value)))
        (`TextRenderComponent.K2_SetText` (`self.TextRender`) (`KismetTextLibrary.Conv_StringToText` _output_get)))
      (:`then_2`
        (if (`self.IsOnCallWithExtension?`)
          (`self.ProcessExtensionSeq`)
          (elif (== (`AudioComponent.Sound` (`self.Audio`)) "/Game/Sounds/Puzzle/Phone/Dial_Tone.Dial_Tone")
            (`AudioComponent.SetSound` _audio "/Game/Sounds/Puzzle/Phone/Dial_Tone.Dial_Tone")
            (`AudioComponent.FadeIn` _audio 6.0 1.0 0.0)))))))

(fn `UserConstructionScript`)