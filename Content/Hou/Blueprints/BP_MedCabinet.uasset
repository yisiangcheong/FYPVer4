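; Interactable medicine cabinet whose cover swings open once, as part of a cigarette-finding puzzle.
; Interaction locks further use and plays a timeline that yaws the cover axle, with interaction status reported from that lock flag.
; CigarreteFound, called from BP_SoapBox, completes the linked door puzzle and reverses the timeline to close the cover.
; A last-puzzle counter macro, comparing against a parameter collection value, is present but never runs.
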(event `/Game/Hou/Blueprints/Interface_Interaction.OnInteracted`
  (set `self.CanBeInteracted?` false) ; To prevent the player from interacting with it again which will cause it to play open anim.
  (bind (_direction _coverrelativeyaw) (`Timeline|CoverOpenAnim` :!via `PlayFromStart` :!label _label)
    (:`Update`
      (`SceneComponent.K2_SetRelativeRotation` (`self.CoverAxle`) (`KismetMathLibrary.MakeRotator` 0.0 0.0 _coverrelativeyaw) false false))))

(event `Cigarrete Found`
  (`/Game/Hou/Blueprints/BP_LockedDoorPuzzle.Puzzle Complete` (`self.DoorPuzzleRef`))
  (set `self.CanBeInteracted?` false)
  (goto _label :!via `Reverse`))

(fn `GetInteractionStatus`
  (returns (`Interaction Status` :type "/Game/Hou/Blueprints/Enum_InteractionStatus Enum"))
  (if (`self.CanBeInteracted?`)
    (return "NewEnumerator1")
    (else
      (return "NewEnumerator0"))))

(fn `UserConstructionScript`)