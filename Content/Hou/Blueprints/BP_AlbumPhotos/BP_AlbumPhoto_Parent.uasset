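; Parent Blueprint for a clickable photo piece in the album puzzle, spawned as a child actor of BP_AlbumPuzzle.
; On BeginPlay it caches its parent actor as the owning puzzle.
; Interactions are forwarded to that puzzle, and clicking the photo mesh asks the puzzle to grab this photo unless it is already the held one.
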(event `self.ReceiveBeginPlay`
  (bind _asbp_album_puzzle (cast `/Game/Hou/Blueprints/BP_AlbumPuzzle` (`self.GetParentActor`)))
  (set `self.AlbumPuzzle` _asbp_album_puzzle))

(event `/Game/Hou/Blueprints/Interface_Interaction.OnInteracted`
  ;[1 1 1] Redirect to interact with the album puzzle
  (`/Game/Hou/Blueprints/BP_NotePuzzle.OnInteracted` (`self.AlbumPuzzle`)))

(event `self.PhotoMesh.OnClicked`
  (params (TouchedComponent :type "PrimitiveComponent Object Reference") (ButtonPressed :type "Key Structure"))
  (bind _albumpuzzle (`self.AlbumPuzzle`))
  (`/Engine/EditorBlueprintResources/StandardMacros.IsValid` _albumpuzzle
    (:`Is Valid`
      (if (!= (`/Game/Hou/Blueprints/BP_AlbumPuzzle.HoldingPhoto` _albumpuzzle) self)
        (`/Game/Hou/Blueprints/BP_AlbumPuzzle.GrabPhoto` _albumpuzzle self 2)))))

(fn `UserConstructionScript`)