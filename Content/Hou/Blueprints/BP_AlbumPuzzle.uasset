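; Photo album puzzle pawn: after a first interaction triggers its memory portal, the player possesses it to arrange photos in album slots.
; Timelines blend the camera around album animations while photos follow the deprojected mouse.
; Released photos snap to nearby slots, swapping occupants; correct ones lock and play narration, wrong ones random hints, with subtitles gating input.
; Once all match, finished dialogue closes the album, returns control and plays a closing cue before the portal closes.
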(event `self.ReceiveBeginPlay`
  (set `self.CameraOriPos` (`SceneComponent.K2_GetComponentToWorld` (`self.Camera`)))
  (for _array_element _
    (`self.SetActorEnableCollision` _array_element false)
    (`self.SetActorHiddenInGame` _array_element true))
  (for (_array_element_2 _array_index) (`self.EmptySpaces`)
    (switch `int` _array_index
      (:`0`
        (`self.SetSceneComponentRefs` _array_index (`self.EmptySpace0`) _array_element_2))
      (:`1`
        (`self.SetSceneComponentRefs` _array_index (`self.EmptySpace1`) _array_element_2))
      (:`2`
        (`self.SetSceneComponentRefs` _array_index (`self.EmptySpace2`) _array_element_2))
      (:`3`
        (`self.SetSceneComponentRefs` _array_index (`self.EmptySpace3`) _array_element_2))
      (:`4`
        (`self.SetSceneComponentRefs` _array_index (`self.EmptySpace4`) _array_element_2))
      (:`5`
        (`self.SetSceneComponentRefs` _array_index (`self.EmptySpace5`) _array_element_2))))
  ;[1 1 1] For use in camera animation
  (set `self.CameraOriginalOffset` (`SceneComponent.RelativeLocation` (`self.Camera`)))
  (`PrimitiveComponent.SetCollisionEnabled` (`self.album_collider_left`) "NoCollision"))

(event `Key|LeftMouseButton`
  (params (Key :type "Key Structure"))
  (:`Released`
    (`self.ReleasePhoto`)
    (for _array_element (`self.EmptySpaces`)
      (bind _output_get (set `self.Win?` (`.HasCorrectPhoto?_6_DFBFDAA44DFBA548284FAABE87BFFA0F` (break `/Game/Hou/Blueprints/BP_AlbumPhotos/Struct_AlbumEmptySpace` _array_element))))
      (if (not _output_get)
        (break)))))

(event `self.ReceiveTick`
  (params (DeltaSeconds :type "Float (single-precision)"))
  (bind _holdingphoto (`self.HoldingPhoto`))
  (bind (_worldlocation _worlddirection) (`PlayerController.DeprojectMousePositionToWorld` (`GameplayStatics.GetPlayerController` 0)))
  (bind (_returnvalue_x _returnvalue_y _returnvalue_z) (`KismetMathLibrary.BreakVector` (`self.K2_GetActorLocation` _holdingphoto)))
  (bind (_returnvalue_x_2 _returnvalue_y_2) (`KismetMathLibrary.BreakVector` (+ _worldlocation (* _worlddirection 40.0))))
  (if (== (`GameplayStatics.GetPlayerPawn` 0) self)
    (`|ExecutionSequence`
      (:`then_0`
        (if (`self.ArePhotosMovable?`)
          (`/Engine/EditorBlueprintResources/StandardMacros.IsValid` (`self.HoldingPhoto`)
            (:`Is Valid`
              (`self.K2_SetActorLocation` _holdingphoto (`KismetMathLibrary.MakeVector` _returnvalue_x_2 _returnvalue_y_2 _returnvalue_z) false false))))))))

(event `/Game/Hou/Blueprints/Interface_Interaction.OnInteracted`
  (bind _returnvalue (`GameplayStatics.GetPlayerController` 0))
  ;[1 1 1] Alex's book disabled
  (bind _asnew_player_controller (cast `/Game/Alex/NewPlayerController` (`GameplayStatics.GetPlayerController` 0)))
  (set `/Game/Alex/NewPlayerController.InPuzzle` true _asnew_player_controller)
  (if (`self.FirstInteract`)
    ;[1 1 1] React when the player points and clicked on the album.
    (if (`self.CanBeInteracted?`)
      (set `self.PlayerCamOriPos` (`SceneComponent.K2_GetComponentToWorld` (`PlayerCameraManager.TransformComponent` (`GameplayStatics.GetPlayerCameraManager` 0))))
      (set `self.PlayerPawnReference` (`Controller.K2_GetPawn` (`GameplayStatics.GetPlayerController` 0)))
      (`Controller.Possess` _returnvalue self)
      ;[1 1 1] Camera Lerp
      (bind (_direction _lerpfloat) (`Timeline|Timeline_0` :!via `PlayFromStart`)
        (:`Update`
          (`SceneComponent.K2_SetWorldTransform` (`self.Camera`) (`KismetMathLibrary.TLerp` (`SceneComponent.K2_GetComponentToWorld` (`PlayerCameraManager.TransformComponent` (`GameplayStatics.GetPlayerCameraManager` 0))) (`self.CameraOriPos`) _lerpfloat) false false))
        (:`Finished`
          (set `PlayerController.bShowMouseCursor` true _returnvalue)
          (`WidgetBlueprintLibrary.SetInputMode_GameAndUIEx` _returnvalue null "DoNotLock" false)
          (set `PlayerController.bEnableMouseOverEvents` true _returnvalue)
          (`PrimitiveComponent.SetCollisionEnabled` (`self.album_collider_right`) "NoCollision")
          (`PrimitiveComponent.SetCollisionEnabled` (`self.album_collider_left`) "NoCollision")
          (bind _asphoto_album_anim_blueprint (cast `/Game/Alex/LiHou_Album/Photo_Album_Anim_Blueprint` (`SkeletalMeshComponent.GetAnimInstance` (`self.photo_album_test2`))))
          (`/Game/Alex/LiHou_Album/Photo_Album_Anim_Blueprint.OpenAlbumAim` _asphoto_album_anim_blueprint)
          ;[1 1 1] A simple camera translate animation to match the album open animation
          (if (not (`self.isAlbumOpened?`))
            (bind (_direction_2 _leftcolliderlerp _positionoffset) (`Timeline|CameraTween` :!via `PlayFromStart`)
              (:`Update`
                (`SceneComponent.K2_SetRelativeLocation` (`self.Camera`) (+ (`self.CameraOriginalOffset`) _positionoffset) false false)
                ;[1 1 1] Move the left collider from right collider's location to the left side when the book opens
                (`SceneComponent.K2_SetRelativeLocation` (`self.album_collider_left`) (`KismetMathLibrary.VLerp` (0.0 0.0 2.0) (-30.5 0.0 2.0) _leftcolliderlerp) false false))
              (:`Finished`
                (set `self.isAlbumOpened?` true)
                (set `self.CameraOriPos` (`SceneComponent.K2_GetComponentToWorld` (`self.Camera`)))))))))
    (else
      (set `self.FirstInteract` true)
      (`/Game/Siang/ItemClass/MemoryContainer_BP.FirstInteract` (`self.MemoryPortal`))
      (`self.SetActorEnableCollision` (`self.SubtitleActor`) true))))

(event `Key|Escape`
  (params (Key :type "Key Structure"))
  (:`Released`
    ;[1 1 1] Camera Lerp Reverse
    (bind (_direction _lerpfloat) (`Timeline|Timeline_2` :!via `ReverseFromEnd`)
      (:`Update`
        (`SceneComponent.K2_SetWorldTransform` (`self.Camera`) (`KismetMathLibrary.TLerp` (`self.PlayerCamOriPos`) (`self.CameraOriPos`) _lerpfloat) false false))
      (:`Finished`
        (`self.ExitPuzzle`)))))

(event `self.ReceiveUnpossessed`
  (params (OldController :type "Controller Object Reference"))
  ;[1 1 1] To prevent a bug where the puzzle is exit with a photo piece being held
  (`self.ReleasePhoto`)
  ;[1 1 1] Re-enable the album collider so that the player can interact with it again after quitting the puzzle
  (if (`self.CanBeInteracted?`)
    (`PrimitiveComponent.SetCollisionEnabled` (`self.album_collider_right`) "QueryAndPhysics")
    (if (`self.isAlbumOpened?`)
      (`PrimitiveComponent.SetCollisionEnabled` (`self.album_collider_left`) "QueryAndPhysics"))))

(event `/Game/Hou/Blueprints/Interface_PuzzleUpdate.OnDialogueFinished`
  (bind _subtitleactor (`self.SubtitleActor`))
  (`AudioComponent.FadeOut` (`self.AmbientAudio`) 1.8 0.0)
  (if (and (`self.Win?`) (`self.CanBeInteracted?`))
    (bind _asphoto_album_anim_blueprint (cast `/Game/Alex/LiHou_Album/Photo_Album_Anim_Blueprint` (`SkeletalMeshComponent.GetAnimInstance` (`self.photo_album_test2`))))
    (`/Game/Alex/LiHou_Album/Photo_Album_Anim_Blueprint.CloseAlbumAnim` _asphoto_album_anim_blueprint)
    (set `self.isAlbumOpened?` false)
    (`KismetSystemLibrary.Delay` 1.5)
    (`SceneComponent.SetVisibility` (`self.Photos`) false true) ; Hide all the photos when the album is closing
    ;[1 1 1] Win logic
    (`KismetSystemLibrary.Delay` 0.4)
    (set `self.CanBeInteracted?` false)
    ;[1 1 1] Camera Lerp Reverse
    (bind (_direction _lerpfloat) (`Timeline|Timeline_1` :!via `ReverseFromEnd`)
      (:`Update`
        (`SceneComponent.K2_SetWorldTransform` (`self.Camera`) (`KismetMathLibrary.TLerp` (`self.PlayerCamOriPos`) (`self.CameraOriPos`) _lerpfloat) false false))
      (:`Finished`
        (`self.ExitPuzzle`)
        (`/Game/Siang/Dialogue/Subtitle_BP.DialogueEnable` _subtitleactor self 2 0.0)
        (`/Game/Siang/Dialogue/Subtitle_BP.PlayClosingCue` _subtitleactor)
        ;[1 1 1] Alex's book enabled(put at end of Sequence or Win logic)
        (bind _asnew_player_controller (cast `/Game/Alex/NewPlayerController` (`GameplayStatics.GetPlayerController` 0)))
        (set `/Game/Alex/NewPlayerController.InPuzzle` false _asnew_player_controller)))
    (elif (== (`/Game/Siang/Dialogue/Subtitle_BP.Conversation_ID` (`self.SubtitleActor`)) 2)
      (`PrimitiveComponent.SetCollisionEnabled` (`/Game/Siang/Dialogue/Subtitle_BP.Box` (`self.SubtitleActor`)) "NoCollision")
      (`/Game/Siang/ItemClass/MemoryContainer_BP.Close` (`self.MemoryPortal`))
      (`KismetSystemLibrary.Delay` 1.0)
      (`self.SetActorHiddenInGame` true)
      (`self.SetActorEnableCollision` false)
      (`ActorComponent.Deactivate` (`Emitter.ParticleSystemComponent` (`self.EmitterAlbum`)))
      (message `/Game/Hou/Blueprints/Interface_PuzzleUpdate.OnClosingClueEnded` (`self.PlayerPawnReference`) "NewEnumerator5")
      (else
        ;[1 1 1] Show the mouse cursor and the holding photo (previously hidden in "ReleasePhoto" function so that the player knows that input is re-enabled.
        (set `PlayerController.bShowMouseCursor` true (`GameplayStatics.GetPlayerController` 0))
        (`self.SetActorHiddenInGame` (`self.HoldingPhoto`) false)))))

(fn `ExitPuzzle`
  (bind _returnvalue (`GameplayStatics.GetPlayerController` 0))
  (if (not (`/Game/Siang/Dialogue/Subtitle_BP.SubtitlesOn` (`self.SubtitleActor`)))
    (`Controller.Possess` _returnvalue (`self.PlayerPawnReference`))
    (set `PlayerController.bShowMouseCursor` false _returnvalue)
    (`WidgetBlueprintLibrary.SetInputMode_GameOnly` _returnvalue)
    (set `PlayerController.bEnableMouseOverEvents` false _returnvalue)))

(fn `GetInteractionStatus`
  (returns (`Interaction Status` :type "/Game/Hou/Blueprints/Enum_InteractionStatus Enum"))
  (if (`self.FirstInteract`)
    (if (`self.CanBeInteracted?`)
      (return "NewEnumerator1")
      (else
        (return "NewEnumerator0")))
    (else
      (return "NewEnumerator2"))))

(fn `GrabPhoto`
  (params (Photo :type "/Game/Hou/Blueprints/BP_AlbumPhotos/BP_AlbumPhoto_Parent Object Reference") (ReleaseDelay :type Integer))
  (bind _ambientaudio (`self.AmbientAudio`))
  (if (`self.ArePhotosMovable?`)
    ;[1 1 1] Grab the clicked on photo
    (set `self.ReleaseCounter` ReleaseDelay)
    (bind _output_get (set `self.HoldingPhoto` Photo))
    (`self.K2_AddActorWorldOffset` _output_get (`KismetMathLibrary.MakeVector` 0.0 0.0 (`self.GrabZOffset`)) false false)
    ;[1 1 1] Play the atmospheric noise of the grab photo
    (`AudioComponent.SetSound` _ambientaudio (`/Game/Hou/Blueprints/BP_AlbumPhotos/BP_AlbumPhoto_Parent.AmbientNoise` (`self.HoldingPhoto`)))
    (`AudioComponent.FadeIn` _ambientaudio 2.0 1.0 0.0)
    ;[1 1 1] Unregister the grabbed photo from the spaces.
    (for (_array_element _array_index) (`self.EmptySpaces`)
      (if (== (`.PhotoSlotted_9_2AB2CC714C071ED4DA1E99BD03592100` (break `/Game/Hou/Blueprints/BP_AlbumPhotos/Struct_AlbumEmptySpace` _array_element)) (`self.HoldingPhoto`))
        (bind _structout (setmembers `/Game/Hou/Blueprints/BP_AlbumPhotos/Struct_AlbumEmptySpace` :`StructRef` _array_element :`HasCorrectPhoto?` false :`PhotoSlotted` null))
        (`KismetArrayLibrary.Array_Set` (`self.EmptySpaces`) _array_index _structout)
        (break)))))

(fn `ReleasePhoto`
  (locals (Local_FilledSpace :type "/Game/Hou/Blueprints/BP_AlbumPhotos/Struct_AlbumEmptySpace Structure") (Local_FilledSpaceIndex :type Integer) (Local_ReleasedPhoto :type "/Game/Hou/Blueprints/BP_AlbumPhotos/BP_AlbumPhoto_Parent Object Reference"))
  (bind _holdingphoto (`self.HoldingPhoto`))
  (bind _local_releasedphoto (`local.Local_ReleasedPhoto`))
  (bind _ambienthintarray (`self.AmbientHintArray`))
  (bind (_local_filledspace_scenetransform _local_filledspace_hascorrectphoto_ _local_filledspace_photoslotted) (break `/Game/Hou/Blueprints/BP_AlbumPhotos/Struct_AlbumEmptySpace` (`local.Local_FilledSpace`)))
  (bind _subtitleactor (`self.SubtitleActor`))
  (bind _ambientaudio (`self.AmbientAudio`))
  (bind _subtitleactor_2 (`self.SubtitleActor`))
  (bind _subtitleactor_3 (`self.SubtitleActor`))
  (bind _subtitleaudio (`self.SubtitleAudio`))
  (bind _local_releasedphoto_2 (`local.Local_ReleasedPhoto`))
  (if (`self.ArePhotosMovable?`)
    ;[1 1 1] Release the grabbed photo (?)
    (if (> (`self.ReleaseCounter`) 0)
      (`/Engine/EditorBlueprintResources/StandardMacros.DecrementInt` (`self.ReleaseCounter`)
        (:`  `
          (if (<= (`self.ReleaseCounter`) 0)
            (`/Engine/EditorBlueprintResources/StandardMacros.IsValid` (`self.HoldingPhoto`)
              (:`Is Valid`
                (set `local.Local_ReleasedPhoto` _holdingphoto)
                (`self.K2_AddActorWorldOffset` _holdingphoto (`KismetMathLibrary.MakeVector` 0.0 0.0 (- 0.0 (`self.GrabZOffset`))) false false)
                (set `self.HoldingPhoto` null)
                (`AudioComponent.Stop` (`self.AmbientAudio`)) ; Stop the ambient noise of the grabbed photo
                (for (_array_element _array_index) (`self.EmptySpaces`)
                  (set `local.Local_FilledSpaceIndex` _array_index)
                  (bind _output_get (set `local.Local_FilledSpace` _array_element))
                  ;[1 1 1] Snap the recently released photo to an empty space if it's close to any of the spaces and the space doesn't filled with a correct photo.
                  (if (not (`.HasCorrectPhoto?_6_DFBFDAA44DFBA548284FAABE87BFFA0F` (break `/Game/Hou/Blueprints/BP_AlbumPhotos/Struct_AlbumEmptySpace` _output_get)))
                    (bind _returnvalue (`SceneComponent.K2_GetComponentLocation` (break `/Game/Hou/Blueprints/BP_AlbumPhotos/Struct_AlbumEmptySpace` _output_get)))
                    (if (<= (`KismetMathLibrary.Vector_DistanceSquared` (`self.K2_GetActorLocation` (`local.Local_ReleasedPhoto`)) _returnvalue) (`KismetMathLibrary.Square` (`self.DistTolerance`)))
                      (`self.K2_SetActorLocation` (`local.Local_ReleasedPhoto`) _returnvalue false false)
                      ;[1 1 1] A photo was snapped to one of the spaces. If there is another photo on that space, grab the other photo.
                      (`/Engine/EditorBlueprintResources/StandardMacros.IsValid` _local_filledspace_photoslotted
                        (:`Is Valid`
                          (`self.GrabPhoto` _local_filledspace_photoslotted 1))
                        (:`Is Not Valid`
                          _))
                      ;[1 1 1] Update the status of the recently occupied space.
                      (bind _structout (setmembers `/Game/Hou/Blueprints/BP_AlbumPhotos/Struct_AlbumEmptySpace` :`StructRef` (`local.Local_FilledSpace`) :`HasCorrectPhoto?` (== (`/Game/Hou/Blueprints/BP_AlbumPhotos/BP_AlbumPhoto_Parent.CorrectSpaceIndex` _local_releasedphoto_2) (`local.Local_FilledSpaceIndex`)) :`PhotoSlotted` _local_releasedphoto_2))
                      (`KismetArrayLibrary.Array_Set` (`self.EmptySpaces`) (`local.Local_FilledSpaceIndex`) _structout)
                      (if (== (`/Game/Hou/Blueprints/BP_AlbumPhotos/BP_AlbumPhoto_Parent.CorrectSpaceIndex` (`local.Local_ReleasedPhoto`)) (`local.Local_FilledSpaceIndex`))
                        (`PrimitiveComponent.SetCollisionEnabled` (`/Game/Hou/Blueprints/BP_AlbumPhotos/BP_AlbumPhoto_Parent.PhotoMesh` (`local.Local_ReleasedPhoto`)) "PhysicsOnly") ; To prevent the photo from being grabbed again bcoz it will trigger the audio cue to play again.
                        ;[1 1 1] The released photo is placed on the right space. Play audio cue, show subtitles
                        (`AudioComponent.SetSound` _subtitleaudio (`/Game/Hou/Blueprints/BP_AlbumPhotos/BP_AlbumPhoto_Parent.AudioCue` (`local.Local_ReleasedPhoto`)))
                        (`AudioComponent.Play` _subtitleaudio 0.0)
                        ;[1 1 1] Show subtitles
                        (`/Game/Siang/Dialogue/Subtitle_BP.DialogueEnable` _subtitleactor_2 self (`/Game/Hou/Blueprints/BP_AlbumPhotos/BP_AlbumPhoto_Parent.ConversationID` _local_releasedphoto) 0.0)
                        ;[1 1 1] Play the corresponding atmospheric noise
                        (set `/Game/Siang/Dialogue/Subtitle_BP.SubArrayInt` (`/Game/Hou/Blueprints/BP_AlbumPhotos/BP_AlbumPhoto_Parent.SubIntervalInt` _local_releasedphoto) _subtitleactor_2)
                        (`AudioComponent.SetSound` _ambientaudio (`/Game/Hou/Blueprints/BP_AlbumPhotos/BP_AlbumPhoto_Parent.AmbientNoise` _local_releasedphoto))
                        (`AudioComponent.Play` _ambientaudio 0.0)
                        (else
                          ;[1 1 1] The photo is incorrect
                          (`/Game/Siang/Dialogue/Subtitle_BP.DialogueEnable` _subtitleactor self (`KismetMathLibrary.RandomIntegerInRange` 9 13) 0.0)
                          (switch `int` (`/Game/Siang/Dialogue/Subtitle_BP.Conversation_ID` _subtitleactor)
                            (:`9`
                              (`GameplayStatics.PlaySound2D` (`|GetArrayItem` _ambienthintarray) 1.0 1.0 0.0 null null)
                              (set `/Game/Siang/Dialogue/Subtitle_BP.SubArrayInt` 39 _subtitleactor_3))
                            (:`10`
                              (`GameplayStatics.PlaySound2D` (`|GetArrayItem` _ambienthintarray 1) 1.0 1.0 0.0 null null)
                              (set `/Game/Siang/Dialogue/Subtitle_BP.SubArrayInt` 40 _subtitleactor_3))
                            (:`11`
                              (`GameplayStatics.PlaySound2D` (`|GetArrayItem` _ambienthintarray 2) 1.0 1.0 0.0 null null)
                              (set `/Game/Siang/Dialogue/Subtitle_BP.SubArrayInt` 41 _subtitleactor_3))
                            (:`12`
                              (`GameplayStatics.PlaySound2D` (`|GetArrayItem` _ambienthintarray 3) 1.0 1.0 0.0 null null)
                              (set `/Game/Siang/Dialogue/Subtitle_BP.SubArrayInt` 42 _subtitleactor_3))
                            (:`13`
                              (`GameplayStatics.PlaySound2D` (`|GetArrayItem` _ambienthintarray 4) 1.0 1.0 0.0 null null)
                              (set `/Game/Siang/Dialogue/Subtitle_BP.SubArrayInt` 43 _subtitleactor_3)))))
                      ;[1 1 1] Hide the mouse cursor and the holding photo so that the player knows that input is disabled.
                      (set `PlayerController.bShowMouseCursor` false (`GameplayStatics.GetPlayerController` 0))
                      (`self.SetActorHiddenInGame` (`self.HoldingPhoto`) true)
                      (break))))))))))))

(fn `SetSceneComponentRefs`
  (params (ItemIndex :type Integer) (SceneComponent :type "SceneComponent Object Reference") (Item :type "/Game/Hou/Blueprints/BP_AlbumPhotos/Struct_AlbumEmptySpace Structure"))
  (bind _structout (setmembers `/Game/Hou/Blueprints/BP_AlbumPhotos/Struct_AlbumEmptySpace` :`StructRef` Item :`SceneTransform` SceneComponent))
  (`KismetArrayLibrary.Array_Set` (`self.EmptySpaces`) ItemIndex _structout))

(fn `UserConstructionScript`)