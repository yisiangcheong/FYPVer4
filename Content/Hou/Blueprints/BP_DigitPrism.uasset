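; BP_DigitPrism is a rotating digit dial on a briefcase combination lock, attached to a parent BP_BriefCase.
; Cursor hover over its collider registers it as the briefcase's current prism and toggles a custom-depth stencil highlight on the dial mesh.
; RotateVertically plays a timeline that rolls the axle opposite the scroll direction, ignoring input mid-animation.
; When finished, it updates the digit, wrapping between 0 and 9, and spawns an attached rotary sound.
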(event `self.ReceiveBeginPlay`
  (set `self.RollTracker` 0.0)
  (bind _asbp_brief_case (cast `/Game/Hou/Blueprints/BP_BriefCase` (`self.GetAttachParentActor`)))
  (set `self.Briefcase` _asbp_brief_case))

(event `self.dial_block_box_collider.OnBeginCursorOver`
  (params (TouchedComponent :type "PrimitiveComponent Object Reference"))
  (bind _briefcase_animated_briefcase_dial_lp (`self.briefcase_animated_briefcase_dial_lp`))
  (`/Game/Hou/Blueprints/BP_BriefCase.SetCurrentPrism` (`self.Briefcase`) self)
  (`PrimitiveComponent.SetRenderCustomDepth` _briefcase_animated_briefcase_dial_lp true)
  (`PrimitiveComponent.SetCustomDepthStencilValue` _briefcase_animated_briefcase_dial_lp 222))

(event `self.dial_block_box_collider.OnEndCursorOver`
  (params (TouchedComponent :type "PrimitiveComponent Object Reference"))
  (bind _briefcase_animated_briefcase_dial_lp (`self.briefcase_animated_briefcase_dial_lp`))
  (`/Game/Hou/Blueprints/BP_BriefCase.SetCurrentPrism` (`self.Briefcase`) null)
  (`PrimitiveComponent.SetRenderCustomDepth` _briefcase_animated_briefcase_dial_lp false)
  (`PrimitiveComponent.SetCustomDepthStencilValue` _briefcase_animated_briefcase_dial_lp 0))

(event `RotateVertically`
  (params (Direction :type Integer))
  (bind _axle (`self.Axle`))
  (bind _relativerotation_roll (`KismetMathLibrary.BreakRotator` (`SceneComponent.RelativeRotation` (`self.Axle`))))
  (bind (_relativerotation_roll_2 _relativerotation_pitch _relativerotation_yaw) (`KismetMathLibrary.BreakRotator` (`SceneComponent.RelativeRotation` _axle)))
  (if (not (`TimelineComponent.IsPlaying` (`self.RotateDialAnim`)))
    (set `self.RollTracker` _relativerotation_roll)
    ;[1 1 1] Mouse wheel scrolling direction is inverse to the actual axle roll rotation. If direction is positive, rotation along x axis is negative, value to add is positive.
    (bind (_direction _rolltoadd) (`Timeline|RotateDialAnim` :!via `PlayFromStart`)
      (:`Update`
        (`SceneComponent.K2_SetRelativeRotation` _axle (`KismetMathLibrary.MakeRotator` (+ (`self.RollTracker`) (* _rolltoadd (* Direction -1.0))) _relativerotation_pitch _relativerotation_yaw) false false))
      (:`Finished`
        (`self.UpdateValue` Direction)
        (`GameplayStatics.SpawnSoundAttached` "/Game/Audio/rotary_code_sfx-01.rotary_code_sfx-01" (`self.RotateSfx`) "None" (0.0 0.0 0.0) (struct) "KeepRelativeOffset" false 1.0 1.0 0.0 null null) ; Used 'spawn sound attached' instead of 'play' because it sounds better when the code is rotated continuously.
      ))))

(fn `UpdateValue`
  (params (ValueToAdd :type Integer))
  (set `self.Value` (+ (`self.Value`) ValueToAdd))
  (if (< (`self.Value`) 0)
    (set `self.Value` 9)
    (elif (> (`self.Value`) 9)
      (set `self.Value` 0))))

(fn `UserConstructionScript`)