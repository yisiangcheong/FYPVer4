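; Parent pawn for inspectable med items that, on interaction, takes possession from the player, matches the first-person camera view and shows a focus widget with the item's subtitle.
; A SceneCapture2D renders only the item to a render texture, recapturing as movement axes or widget mouse drags spin MeshPivot, leaving the cameras still.
; Closing the widget restores player possession and the mesh transform; OpenItem is an empty hook for children like BP_SoapBox.
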(event `/Game/Hou/Blueprints/Interface_Interaction.OnInteracted`
  (bind _returnvalue (`GameplayStatics.GetPlayerController` 0))
  (bind _returnvalue_2 (`GameplayStatics.GetPlayerController` 0))
  (bind _scenecapturecomponent2d (`self.SceneCaptureComponent2D`))
  (set `self.DefaultMeshPivotXForm` (`SceneComponent.K2_GetComponentToWorld` (`self.Mesh_Pivot`)))
  ;[1 1 1] Setup to capture only this actor into the render texture "ItemRenderTarget"
  (set `SceneCaptureComponent.ShowOnlyActors` (`|MakeArray` self :!type "Actor Object Reference") _scenecapturecomponent2d)
  (`SceneCaptureComponent2D.CaptureScene` _scenecapturecomponent2d)
  (set `self.PlayerPawnReference` (`Controller.K2_GetPawn` _returnvalue))
  (`Controller.Possess` _returnvalue self) ; Possess this pawn to disable the controls of player character
  (set `PlayerController.bShowMouseCursor` true _returnvalue_2)
  (`WidgetBlueprintLibrary.SetInputMode_GameAndUIEx` _returnvalue_2 null "DoNotLock" false)
  ;[1 1 1] Set this pawn's camera transform to the transform of the player character's fpsCamera so it looks like we are viewing from the player point of view.
  (bind _asbp_player_character (cast `/Game/Hou/Blueprints/BP_PlayerCharacter` (`self.PlayerPawnReference`)))
  (`SceneComponent.K2_SetWorldTransform` (`self.Camera`) (`SceneComponent.K2_GetComponentToWorld` (`/Game/Hou/Blueprints/BP_PlayerCharacter.FirstPersonCamera` _asbp_player_character)) false false)
  ;[1 1 1] Show/create widget
  (`/Engine/EditorBlueprintResources/StandardMacros.IsValid` (`self.FocusWidgetRef`)
    (:`Is Valid`
      _)
    (:`Is Not Valid`
      (bind _returnvalue_3 (`|CreateWidget` "/Game/Hou/Widgets/Widget_MedItemFocus.Widget_MedItemFocus_C"))
      (set `self.FocusWidgetRef` _returnvalue_3)))
  (`UserWidget.AddToViewport` (`self.FocusWidgetRef`) 0)
  ;[1 1 1] Show the text describing this item.
  (`TextBlock.SetText` (`/Game/Hou/Widgets/Widget_MedItemFocus.Subtitle` (`self.FocusWidgetRef`)) (`KismetTextLibrary.Conv_StringToText` (`self.Subtitle`))))

(event `CloseWidget`
  (bind _returnvalue (`GameplayStatics.GetPlayerController` 0))
  (`Controller.Possess` _returnvalue (`self.PlayerPawnReference`))
  (set `PlayerController.bShowMouseCursor` false _returnvalue)
  (`WidgetBlueprintLibrary.SetInputMode_GameOnly` _returnvalue)
  (`SceneComponent.K2_SetWorldTransform` (`self.Mesh_Pivot`) (`self.DefaultMeshPivotXForm`) false false))

(event `Open Item`)

(event `self.ReceiveUnpossessed`
  (params (OldController :type "Controller Object Reference"))
  (bind _focuswidgetref (`self.FocusWidgetRef`))
  (`/Engine/EditorBlueprintResources/StandardMacros.IsValid` _focuswidgetref
    (:`Is Valid`
      (`Widget.RemoveFromParent` _focuswidgetref))))

(event `InputAxis|MoveForward`
  (params (AxisValue :type "Float (single-precision)"))
  (`SceneComponent.K2_AddWorldRotation` (`self.Mesh_Pivot`) (`KismetMathLibrary.MakeRotator` 0.0 (* AxisValue (* (`self.SpinningSpeed`) -1.0))) false false)
  (`SceneCaptureComponent2D.CaptureScene` (`self.SceneCaptureComponent2D`)))

(event `InputAxis|MoveRight`
  (params (AxisValue :type "Float (single-precision)"))
  (`SceneComponent.K2_AddWorldRotation` (`self.Mesh_Pivot`) (`KismetMathLibrary.MakeRotator` 0.0 0.0 (* AxisValue (* (`self.SpinningSpeed`) -1.0))) false false)
  (`SceneCaptureComponent2D.CaptureScene` (`self.SceneCaptureComponent2D`)))

(event `MouseClickedOnWidget`
  (params (`Mouse Location` :type "Vector2D Structure"))
  ;[1 1 1] These events are triggered by Widget_MedItemRenderer to rotate mesh with mouse. *Not rotating the whole actor because the action will rotate the cameras as well.
  (set `self.CanRotate?` true))

(event `MouseReleasedFromWidget`
  ;[1 1 1] These events are triggered by Widget_MedItemRenderer to rotate mesh with mouse. *Not rotating the whole actor because the action will rotate the cameras as well.
  (set `self.CanRotate?` false))

(event `MouseMovedOnWidget`
  (params (`Mouse Delta` :type "Vector2D Structure"))
  (bind (_x _y) (`KismetMathLibrary.BreakVector2D` (* `Mouse Delta` 0.4)))
  ;[1 1 1] These events are triggered by Widget_MedItemRenderer to rotate mesh with mouse. *Not rotating the whole actor because the action will rotate the cameras as well.
  (if (`self.CanRotate?`)
    (`SceneComponent.K2_AddWorldRotation` (`self.Mesh_Pivot`) (`KismetMathLibrary.MakeRotator` 0.0 _y (* _x -1.0)) false false)
    (`SceneCaptureComponent2D.CaptureScene` (`self.SceneCaptureComponent2D`))))

(fn `GetInteractionStatus`
  (returns (`Interaction Status` :type "/Game/Hou/Blueprints/Enum_InteractionStatus Enum"))
  (return "NewEnumerator1"))

(fn `UserConstructionScript`)