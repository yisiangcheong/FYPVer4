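; BP_SoapBox is an inspectable soap box item that can be opened to trigger a cigarette discovery in its parent BP_MedCabinet.
; Interacting shows an open button on the focus widget.
; Opening plays a timeline that slides the inner box along Y from its cached closed position, then sets a subtitle.
; Closing the widget snaps the box shut and calls CigarreteFound on the cabinet, whether or not it was opened.
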(event `self.ReceiveBeginPlay`
  (set `self.BoxClosedRelativeLoc` (`SceneComponent.RelativeLocation` (`self.Soap_box_lp_Soap_box_inner_lp001`))))

(event `/Game/Hou/Blueprints/Interface_Interaction.OnInteracted`
  (`parent.OnInteracted`)
  (`/Game/Hou/Widgets/Widget_ItemFocus.ShowOpenButton` (`self.FocusWidgetRef`) true))

(event `self.CloseWidget`
  (`parent.CloseWidget`)
  (`SceneComponent.K2_SetRelativeLocation` (`self.Soap_box_lp_Soap_box_inner_lp001`) (`self.BoxClosedRelativeLoc`) false false)
  (bind _asbp_med_cabinet (cast `/Game/Hou/Blueprints/BP_MedCabinet` (`self.GetParentActor`)))
  (`/Game/Hou/Blueprints/BP_MedCabinet.Cigarrete Found` _asbp_med_cabinet))

(event `self.Open Item`
  (bind (_boxclosedrelativeloc_x _boxclosedrelativeloc_y _boxclosedrelativeloc_z) (`KismetMathLibrary.BreakVector` (`self.BoxClosedRelativeLoc`)))
  (`/Game/Hou/Widgets/Widget_ItemFocus.ShowOpenButton` (`self.FocusWidgetRef`) false)
  (bind (_direction _yoffset) (`Timeline|SoapBoxOpen` :!via `PlayFromStart`)
    (:`Update`
      (`SceneComponent.K2_SetRelativeLocation` (`self.Soap_box_lp_Soap_box_inner_lp001`) (`KismetMathLibrary.MakeVector` _boxclosedrelativeloc_x (+ _boxclosedrelativeloc_y _yoffset) _boxclosedrelativeloc_z) false false))
    (:`Finished`
      (`TextBlock.SetText` (`/Game/Hou/Widgets/Widget_ItemFocus.Subtitle` (`self.FocusWidgetRef`)) "Sigh... Emmie..."))))

(fn `UserConstructionScript`
  (`parent.UserConstructionScript`))