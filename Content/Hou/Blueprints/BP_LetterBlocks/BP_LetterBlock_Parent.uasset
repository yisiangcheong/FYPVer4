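; Parent Blueprint for a flippable letter block in a BP_BlockPuzzle, cached from its attach parent on BeginPlay.
; Cursor hover sets or clears the puzzle's current block, and interaction is forwarded because the puzzle itself cannot be line-traced.
; A timeline lifts and rolls the block, then steps the wrapping letter index and triggers the win check.
; It also offers a letter check, custom-depth outlining and a loop that flips toward the hidden letter's roll.
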(event `self.ReceiveBeginPlay`
  (bind _asbp_block_puzzle (cast `/Game/Hou/Blueprints/BP_BlockPuzzle` (`self.GetAttachParentActor`)))
  (set `self.BlockPuzzle` _asbp_block_puzzle))

(event `self.LetterBlockMesh.OnBeginCursorOver`
  (params (TouchedComponent :type "PrimitiveComponent Object Reference"))
  (`/Game/Hou/Blueprints/BP_BlockPuzzle.SetCurrentBlock` (`self.BlockPuzzle`) self))

(event `self.LetterBlockMesh.OnEndCursorOver`
  (params (TouchedComponent :type "PrimitiveComponent Object Reference"))
  (`/Game/Hou/Blueprints/BP_BlockPuzzle.SetCurrentBlock` (`self.BlockPuzzle`) null))

(event `/Game/Hou/Blueprints/Interface_Interaction.OnInteracted`
  ;[1 1 1] Redirect to interact with the letter block puzzle. BP_BlockPuzzle is intangible, it can't be detected by line tracing.
  (message `/Game/Hou/Blueprints/Interface_Interaction.OnInteracted` (`self.BlockPuzzle`)))

(event `FlipBlockAnim`
  (params (flipDirection :type Integer))
  (bind _meshxform (`self.MeshXForm`))
  (set `self.MeshXForm` (`SceneComponent.K2_GetComponentToWorld` (`self.DefaultSceneRoot`)))
  (bind (_direction _rolltoadd _zpositionoffset) (`Timeline|FlipBlockTimeline` :!via `PlayFromStart`)
    (:`Update`
      (`SceneComponent.K2_SetWorldLocationAndRotation` (`self.DefaultSceneRoot`) (`KismetMathLibrary.MakeVector` (.x (.location _meshxform)) (.y (.location _meshxform)) (+ _zpositionoffset (.z (.location _meshxform)))) (`KismetMathLibrary.MakeRotator` (+ (.roll (.rotation _meshxform)) (* (* flipDirection -1) _rolltoadd)) (.pitch (.rotation _meshxform)) (.yaw (.rotation _meshxform))) false false))
    (:`Finished`
      (`self.UpdateCurrentLetterIndex` flipDirection)
      (`/Game/Hou/Blueprints/BP_BlockPuzzle.CheckWinning` (`self.BlockPuzzle`)))))

(event `FlipToHiddenLetter`
  (bind _returnvalue_roll (`KismetMathLibrary.BreakRotator` (`SceneComponent.K2_GetComponentRotation` (`self.DefaultSceneRoot`))))
  (bind _returnvalue_roll_2 (`KismetMathLibrary.BreakRotator` (`SceneComponent.K2_GetComponentRotation` (`self.DefaultSceneRoot`))))
  (while (> (`KismetMathLibrary.Abs` (- _returnvalue_roll_2 (`self.HiddenLetterRoll`))) 1.0)
    (if (not (`TimelineComponent.IsPlaying` (`self.FlipBlockTimeline`)))
      (`self.FlipBlockAnim` (`KismetMathLibrary.FTrunc` (`KismetMathLibrary.SignOfFloat` (- _returnvalue_roll (`self.HiddenLetterRoll`))))))))

(fn `EnableOutline`
  (params (`Outline?` :type Boolean))
  (bind _letterblockmesh (`self.LetterBlockMesh`))
  (if `Outline?`
    (`PrimitiveComponent.SetRenderCustomDepth` _letterblockmesh true)
    (`PrimitiveComponent.SetCustomDepthStencilValue` _letterblockmesh 222)
    (else
      (`PrimitiveComponent.SetRenderCustomDepth` _letterblockmesh false)
      (`PrimitiveComponent.SetCustomDepthStencilValue` _letterblockmesh 0))))

(fn `Flip`
  (params (FlipDirection :type Integer))
  ;[1 1 1] A letter block can only be flipped if its flipping animation is not playing
  (if (not (`TimelineComponent.IsPlaying` (`self.FlipBlockTimeline`)))
    (`self.FlipBlockAnim` FlipDirection)))

(fn `IsLetterCorrect?`
  (params (CorrectLetter :type Name))
  (returns (ReturnValue :type Boolean))
  (return (== CorrectLetter (`|GetArrayItem` (`self.AllLetters`) (`self.CurrentLetterIndex`)))))

(fn `UpdateCurrentLetterIndex`
  (params (ValueToAdd :type Integer))
  (bind _output_get (set `self.CurrentLetterIndex` (+ (`self.CurrentLetterIndex`) ValueToAdd)))
  (if (>= _output_get (`KismetArrayLibrary.Array_Length` (`self.AllLetters`)))
    (set `self.CurrentLetterIndex` 0)
    (elif (< (`self.CurrentLetterIndex`) 0)
      (set `self.CurrentLetterIndex` (- (`KismetArrayLibrary.Array_Length` (`self.AllLetters`)) 1)))))

(fn `UserConstructionScript`)