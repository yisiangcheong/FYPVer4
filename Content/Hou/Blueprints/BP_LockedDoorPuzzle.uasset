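; Locked-door puzzle pawn where the player wiggles a card down to a target height to open the door.
; Interacting possesses the pawn; Tick maps mouse offset to clamped card tilt, turning pitch changes into decaying friction that lowers the card.
; Clicking rattles the door, or, at target height, drops the card, opens the door, returns control and starts closing dialogue.
; When that dialogue ends, the memory portal closes and the player pawn is notified.
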(event `Key|LeftMouseButton`
  (params (Key :type "Key Structure"))
  (bind _interactable_door_lp (`self.interactable_door_lp`))
  (bind _interactable_door_lp_2 (`self.interactable_door_lp`))
  (bind (_relativelocation_x _relativelocation_y _relativelocation_z) (`KismetMathLibrary.BreakVector` (`SceneComponent.RelativeLocation` (`self.card_pivot`))))
  (bind (_relativerotation_roll _relativerotation_pitch _relativerotation_yaw) (`KismetMathLibrary.BreakRotator` (`SceneComponent.RelativeRotation` (`self.interactable_door_lp`))))
  (bind (_relativerotation_roll_2 _relativerotation_pitch_2 _relativerotation_yaw_2) (`KismetMathLibrary.BreakRotator` (`SceneComponent.RelativeRotation` (`self.interactable_door_lp`))))
  (bind (_relativerotation_roll_3 _relativerotation_pitch_3) (`KismetMathLibrary.BreakRotator` (`SceneComponent.RelativeRotation` _interactable_door_lp)))
  (bind (_relativerotation_roll_4 _relativerotation_pitch_4) (`KismetMathLibrary.BreakRotator` (`SceneComponent.RelativeRotation` _interactable_door_lp_2)))
  ;[1 1 1] Mouse Control
  (:`Released`
    (if (`self.CanBeInteracted`)
      (if (< (`KismetMathLibrary.Abs` (- _relativelocation_z (`self.TargetCardZLoc`))) 0.5)
        (if (not (`TimelineComponent.IsPlaying` (`self.Door Opens Anim`)))
          ;[1 1 1] Let the card fall to the ground
          (`PrimitiveComponent.SetSimulatePhysics` (`self.interactable_card_lp`) true)
          (set `self.CachedDoorYaw` _relativerotation_yaw_2)
          (`|ExecutionSequence`
            (:`then_0`
              (`KismetSystemLibrary.Delay` 0.75)
              (`self.ExitPuzzle`))
            (:`then_1`
              (bind (_direction _newdooryaw) (`Timeline|Door Opens Anim` :!via `PlayFromStart`)
                (:`Update`
                  (`SceneComponent.K2_SetRelativeRotation` _interactable_door_lp_2 (`KismetMathLibrary.MakeRotator` _relativerotation_roll_4 _relativerotation_pitch_4 (+ (`self.CachedDoorYaw`) _newdooryaw)) false false))
                (:`Finished`
                  (set `self.CanBeInteracted` false)
                  (`/Game/Siang/Dialogue/Subtitle_BP.DialogueEnable` (`self.SubtitleActor`) self 2 0.0))))))
        (elif (not (`TimelineComponent.IsPlaying` (`self.Door Locked Anim`)))
          (set `self.CachedDoorYaw` _relativerotation_yaw)
          (bind (_direction_2 _newdooryaw_2) (`Timeline|Door Locked Anim` :!via `PlayFromStart`)
            (:`Update`
              (`SceneComponent.K2_SetRelativeRotation` _interactable_door_lp (`KismetMathLibrary.MakeRotator` _relativerotation_roll_3 _relativerotation_pitch_3 (+ (`self.CachedDoorYaw`) _newdooryaw_2)) false false))))))))

(event `/Game/Hou/Blueprints/Interface_Interaction.OnInteracted`
  (bind _returnvalue (`GameplayStatics.GetPlayerController` 0))
  ;[1 1 1] React when the player points and clicked on the door.
  (if (`self.CanBeInteracted`)
    (set `self.PlayerPawnReference` (`Controller.K2_GetPawn` (`GameplayStatics.GetPlayerController` 0)))
    (`Controller.Possess` _returnvalue self)
    (set `PlayerController.bShowMouseCursor` true _returnvalue)
    (`WidgetBlueprintLibrary.SetInputMode_GameAndUIEx` _returnvalue null "DoNotLock" false)
    (set `PlayerController.bEnableMouseOverEvents` true _returnvalue)))

(event `Key|Escape`
  (params (Key :type "Key Structure"))
  ;[1 1 1] Exit the brief case puzzle
  (:`Released`
    (`self.ExitPuzzle`)))

(event `self.ReceiveTick`
  (params (DeltaSeconds :type "Float (single-precision)"))
  (bind _returnvalue (`GameplayStatics.GetPlayerController` 0))
  (bind _card_pivot (`self.card_pivot`))
  (bind _card_pivot_2 (`self.card_pivot`))
  (bind (_locationx _locationy) (`PlayerController.GetMousePosition` _returnvalue))
  (bind (_relativerotation_roll _relativerotation_pitch) (`KismetMathLibrary.BreakRotator` (`SceneComponent.RelativeRotation` (`self.card_pivot`))))
  (bind (_relativelocation_x _relativelocation_y _relativelocation_z) (`KismetMathLibrary.BreakVector` (`SceneComponent.RelativeLocation` (`self.card_pivot`))))
  (bind (_relativerotation_roll_2 _relativerotation_pitch_2 _relativerotation_yaw) (`KismetMathLibrary.BreakRotator` (`SceneComponent.RelativeRotation` _card_pivot)))
  (bind (_relativerotation_roll_3 _relativerotation_pitch_3) (`KismetMathLibrary.BreakRotator` (`SceneComponent.RelativeRotation` _card_pivot_2)))
  (bind _screenlocation (`PlayerController.ProjectWorldLocationToScreen` _returnvalue (`SceneComponent.K2_GetComponentLocation` (`self.interactable_card_lp`)) false))
  (bind _returnvalue_2 (/ (- (`KismetMathLibrary.BreakVector2D` _screenlocation) _locationx) 20.0))
  (bind _returnvalue_3 (/ (- (`.Y` (`KismetMathLibrary.BreakVector2D` _screenlocation)) _locationy) 5.0))
  (if (== (`GameplayStatics.GetPlayerPawn` 0) self)
    (`|ExecutionSequence`
      (:`then_0`
        (if (and (<= _returnvalue_2 12.0) (>= _returnvalue_2 -6.0))
          (`SceneComponent.K2_SetRelativeRotation` _card_pivot_2 (`KismetMathLibrary.MakeRotator` _relativerotation_roll_3 _relativerotation_pitch_3 _returnvalue_2) false false)))
      (:`then_1`
        (set `self.PrevCardPitch` _relativerotation_pitch)
        (if (and (<= _returnvalue_3 26.0) (>= _returnvalue_3 -26.0))
          (`SceneComponent.K2_SetRelativeRotation` _card_pivot (`KismetMathLibrary.MakeRotator` _relativerotation_roll_2 _returnvalue_3 _relativerotation_yaw) false false)
          (bind _output_get (set `self.CardFriction` (+ (`self.CardFriction`) (`KismetMathLibrary.Abs` (- _returnvalue_3 (`self.PrevCardPitch`))))))
          (if (>= _relativelocation_z (`self.TargetCardZLoc`))
            (`SceneComponent.K2_AddLocalOffset` (`self.card_pivot`) (`KismetMathLibrary.MakeVector` 0.0 0.0 (* (* (/ _output_get 5.0) DeltaSeconds) -1.0)) false false))))
      (:`then_2`
        (set `self.CardFriction` (* (`self.CardFriction`) 0.5))))))

(event `/Game/Hou/Blueprints/Interface_PuzzleUpdate.OnDialogueFinished`
  ;[1 1 1] Closing subs has ended, notify the player, shrink the portal.
  (if (== (`/Game/Siang/Dialogue/Subtitle_BP.Conversation_ID` (`self.SubtitleActor`)) 2)
    (`/Game/Siang/ItemClass/MemoryContainer_BP.Close` (`self.MemoryPortal`))
    (message `/Game/Hou/Blueprints/Interface_PuzzleUpdate.OnClosingClueEnded` (`self.PlayerPawnReference`) "NewEnumerator6")))

(fn `ExitPuzzle`
  (bind _returnvalue (`GameplayStatics.GetPlayerController` 0))
  (`Controller.Possess` _returnvalue (`self.PlayerPawnReference`))
  (set `PlayerController.bShowMouseCursor` false _returnvalue)
  (`WidgetBlueprintLibrary.SetInputMode_GameOnly` _returnvalue)
  (set `PlayerController.bEnableMouseOverEvents` false _returnvalue))

(fn `UserConstructionScript`)