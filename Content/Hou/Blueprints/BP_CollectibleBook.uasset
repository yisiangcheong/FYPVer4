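; Collectible book pickup that the player interacts with to obtain the book.
; Interaction plays a grab sound, hides the actor and disables its collision, then after a short delay calls StandUp on the player character and destroys itself.
; It then sets HaveBook on the player controller and shows a tutorial widget, immediately calling its Disappear.
; GetInteractionStatus always reports one fixed enum value.
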(event `/Game/Hou/Blueprints/Interface_Interaction.OnInteracted`
  (`GameplayStatics.PlaySound2D` "/Game/Calvin_Sounds/SFX/SFX__Book_Grab__190721.SFX__Book_Grab__190721" 1.0 1.0 0.0 null null)
  (bind _asbp_player_character (cast `/Game/Hou/Blueprints/BP_PlayerCharacter` (`Controller.K2_GetPawn` (`GameplayStatics.GetPlayerController` 0))))
  (`self.SetActorHiddenInGame` true)
  (`self.SetActorEnableCollision` false)
  (`KismetSystemLibrary.Delay` 0.2)
  (`/Game/Hou/Blueprints/BP_PlayerCharacter.Stand Up` _asbp_player_character)
  (`self.K2_DestroyActor`)
  (bind _asnew_player_controller (cast `/Game/Alex/NewPlayerController` (`GameplayStatics.GetPlayerController` 0)))
  (set `/Game/Alex/NewPlayerController.HaveBook` true _asnew_player_controller)
  (bind _returnvalue (`|CreateWidget` "/Game/Alex/Tutorial/TutorialWidget.TutorialWidget_C" (`GameplayStatics.GetPlayerController` 0)))
  (`UserWidget.AddToViewport` _returnvalue 0)
  (`/Game/Alex/Tutorial/TutorialWidget.Disappear` _returnvalue))

(fn `GetInteractionStatus`
  (returns (`Interaction Status` :type "/Game/Hou/Blueprints/Enum_InteractionStatus Enum"))
  (return "NewEnumerator1"))

(fn `UserConstructionScript`)