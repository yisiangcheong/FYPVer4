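; BP_Hand is a hand that reaches out as the player holds MoveForward, interrupting a dream with an alarm beep.
; Positive input accumulates a clamped reach timer, which lerps the actor from its initial to final world location with quadratic ease-out.
; Two seconds before the timer maxes out, a one-shot flag triggers the beep and CallInterruptDream.
; The timer only increases, so releasing input pauses the hand without retracting it.
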(event `InputAxis|MoveForward`
  (params (AxisValue :type "Float (single-precision)"))
  (bind _reachoutduration (`self.ReachOutDuration`))
  ;[1 1 1] Input Handling: W key
  (if (> AxisValue 0.0)
    (set `self.ReachOutDuration` (+ _reachoutduration (* AxisValue (`GameplayStatics.GetWorldDeltaSeconds`))))
    (bind _output_get (set `self.ReachOutDuration` (`KismetMathLibrary.FClamp` _reachoutduration 0.0 (`self.MaxReachOutDuration`))))
    (bind _returnvalue (- 1.0 (/ _output_get (`self.MaxReachOutDuration`))))
    (`self.K2_SetActorLocation` (`KismetMathLibrary.VLerp` (`self.FinalWorldLoc`) (`self.InitialWorldLoc`) (* _returnvalue _returnvalue)))
    (if (>= (`self.ReachOutDuration`) (- (`self.MaxReachOutDuration`) 2.0))
      (if (not (`self.DreamInterrupted`))
        (set `self.DreamInterrupted` true)
        (`GameplayStatics.PlaySound2D` "/Game/Audio/AlarmBeep_Cue.AlarmBeep_Cue" 1.0 1.0 0.0 null null)
        (`self.InterruptDream`)))))

(event `self.ReceiveBeginPlay`)

(fn `UserConstructionScript`)