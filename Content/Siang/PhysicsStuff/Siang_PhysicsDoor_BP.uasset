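; Physics door actor that registers its static mesh as the player's grab target when the player character enters its box trigger.
; On overlap it looks up the first Siang_Character and sets that character's GrabTarget to the mesh.
; It also stores the character-to-door distance, converted to a vector, as InteractionDistance and prints a debug message.
; The graph has no end-overlap handling to clear the target.
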(event `self.Box.OnComponentBeginOverlap`
  (params (OverlappedComponent :type "PrimitiveComponent Object Reference") (OtherActor :type "Actor Object Reference") (OtherComp :type "PrimitiveComponent Object Reference") (OtherBodyIndex :type Integer) (bFromSweep :type Boolean) (SweepResult :type "HitResult Structure (by ref)"))
  (if (== OtherActor (`GameplayStatics.GetPlayerCharacter` 0))
    (bind _outactors (`GameplayStatics.GetAllActorsOfClass` "/Game/Siang/Siang_Character.Siang_Character_C"))
    (bind _assiang_character (cast `/Game/Siang/Siang_Character` (`|GetArrayItem` _outactors)))
    (set `/Game/Siang/Siang_Character.GrabTarget` (`self.StaticMesh`) _assiang_character)
    (set `/Game/Siang/Siang_Character.InteractionDistance` (`KismetMathLibrary.Conv_DoubleToVector` (`KismetMathLibrary.VSize` (- (`self.K2_GetActorLocation` _assiang_character) (`self.K2_GetActorLocation`)))) _assiang_character)
    (`KismetSystemLibrary.PrintString` "Set")))

(fn `UserConstructionScript`)