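; Puzzle-completion controller that gates the last memory puzzle and stages the ending reveal.
; BeginPlay disables the last memory's container, item, subtitle collision and particles; TriggerLastPuzzle restores container overlap, item visibility, child collision and particles, and enables its own collision.
; OpenAll toggles all memory containers, unhides all memory items with their child actors, and plays the ending cinematic subtitle.
; Tick also spins FanBlades at a fixed per-frame step.
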(event `OpenAll`
  (for _array_element (`self.AllMemContainers`)
    (`/Game/Siang/ItemClass/MemoryContainer_BP.ToggleMemory` _array_element))
  (for _array_element_2 (`self.AllMemItems`)
    (`self.SetActorHiddenInGame` _array_element_2 false)
    (for _array_element_3 (`self.GetAllChildActors` _array_element_2 true)
      (`self.SetActorHiddenInGame` _array_element_3 false)))
  (`/Game/Siang/Dialogue/Subtitle_BP.ManualPlay` (`self.EndingCinematicSubtitleBP`)))

(event `self.ReceiveBeginPlay`
  (bind _lastmemoryitem (`self.LastMemoryItem`))
  (`self.SetActorEnableCollision` (`self.LastSubtitleBP`) false)
  (`PrimitiveComponent.SetCollisionProfileName` (`/Game/Siang/ItemClass/MemoryContainer_BP.Box` (`self.LastMemoryContainer`)) "NoCollision")
  (`self.SetActorHiddenInGame` _lastmemoryitem true)
  (`self.SetActorEnableCollision` _lastmemoryitem false)
  (for _array_element (`self.GetAllChildActors` _lastmemoryitem true)
    (`self.SetActorEnableCollision` _array_element false))
  (`ActorComponent.Deactivate` (`Emitter.ParticleSystemComponent` (`self.LastParticleEmitter`))))

(event `TriggerLastPuzzle`
  (bind _lastmemoryitem (`self.LastMemoryItem`))
  (`KismetSystemLibrary.PrintString` "Last!")
  (`PrimitiveComponent.SetCollisionProfileName` (`/Game/Siang/ItemClass/MemoryContainer_BP.Box` (`self.LastMemoryContainer`)) "OverlapAllDynamic")
  (`self.SetActorHiddenInGame` _lastmemoryitem false)
  (`self.SetActorEnableCollision` true)
  (for _array_element (`self.GetAllChildActors` _lastmemoryitem true)
    (`self.SetActorEnableCollision` _array_element true))
  (`ActorComponent.Activate` (`Emitter.ParticleSystemComponent` (`self.LastParticleEmitter`)) false))

(event `self.ReceiveTick`
  (params (DeltaSeconds :type "Float (single-precision)"))
  (`self.K2_AddActorWorldRotation` (`self.FanBlades`) (struct :`Yaw` 5.0) false false))

(fn `UserConstructionScript`)