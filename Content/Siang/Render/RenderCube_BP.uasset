(event `self.ReceiveTick`
  (params (DeltaSeconds :type "Float (single-precision)"))
  (bind _disablerender (`self.DisableRender`))
  (bind _cube (`self.Cube`))
  (if (`self.WasRecentlyRendered` 0.4)
    (if (not _disablerender)
      (set `self.DisableRender` true)
      (`SceneComponent.SetVisibility` _cube true false)
      (`KismetSystemLibrary.PrintString` "I See You" true true (struct :`G` 0.66 :`B` 1.0 :`A` 1.0) 1.0))
    (elif _disablerender
      (`SceneComponent.SetVisibility` _cube false false)
      (set `self.DisableRender` false))))

(fn `UserConstructionScript`)