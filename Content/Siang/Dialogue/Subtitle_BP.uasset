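; Trigger-box subtitle actor that shows timed NPC dialogue and plays an opening or closing audio cue, depending on puzzle completion.
; BeginPlay gathers data table rows by NPCID, and lookups select lines by ConversationID and line number.
; Player overlap or DialogueEnable starts playback, and Tick drives line advancement while subtitles are on.
; Widget updates respect the GameInstance subtitle setting; the last line triggers slide-out and notifies the stored caller.
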(event `GetLineFinal`
  (bind _dialoguewidget (`self.DialogueWidget`))
  ;[1 1 1] From DialogueGetLine, moved here for animation delay
  (`/Game/Siang/Dialogue/DialogueWidget.SlideOutAnim` _dialoguewidget)
  (`KismetSystemLibrary.Delay` 0.5)
  (`Widget.RemoveFromParent` _dialoguewidget)
  (set `self.DialogueWidget` null)
  (set `self.LineCurrent` 0)
  (set `self.SubtitlesOn` false)
  (message `/Game/Hou/Blueprints/Interface_PuzzleUpdate.OnDialogueFinished` (`self.CallerRef`)))

(event `PlayClosingCue`
  (bind _audio (`self.Audio`))
  ;[1 1 1] Playing Closing Cue Custom Events
  (`AudioComponent.SetSound` _audio (`self.ClosingCue`))
  (`AudioComponent.FadeIn` _audio 1.0 1.0 0.0))

(event `self.ReceiveBeginPlay`
  ;[1 1 1] Begin Play to Get Data Table
  (`AudioComponent.SetSound` (`self.Audio`) (`self.OpeningCue`))
  (bind _outrownames (`DataTableFunctionLibrary.GetDataTableRowNames` (`self.DialogueDataTable`)))
  (for _array_element _outrownames
    (bind _returnvalue (`|GetDataTableRow` (`self.DialogueDataTable`) _array_element)
      (:`then`
        (if (== (`.NPC_ID_2_E1A2C3CC40E41BED22A7C2A4749AC1E5` (break `/Game/Siang/Dialogue/DialogueStructure` _returnvalue)) (`self.NPC_ID`))
          (`KismetArrayLibrary.Array_Add` (`self.MyDialogue`) _array_element)))))
  (if (`self.ActorHasTag` "BookSub")
    (`PrimitiveComponent.SetCollisionEnabled` (`self.Box`) "NoCollision")))

(event `PlayOpeningCue`
  (bind _audio (`self.Audio`))
  ;[1 1 1] Playing Closing Cue Custom Events
  (`AudioComponent.SetSound` _audio (`self.OpeningCue`))
  (`AudioComponent.FadeIn` _audio 1.0 1.0 0.0))

(event `AudioFadeOut`
  ;[1 1 1] Playing Closing Cue Custom Events
  (`AudioComponent.FadeOut` (`self.Audio`) 1.0 0.0))

(event `self.SubtitleInteract`
  ;[1 1 1] Custom Event Subtitle Interact
  (`/Engine/EditorBlueprintResources/StandardMacros.IncrementInt` (`self.LineCurrent`)
    (:`  `
      (bind _ascustom_game_instance (cast `/Game/Prototype/CustomGameInstance` (`GameplayStatics.GetGameInstance`)))
      (if (`/Game/Prototype/CustomGameInstance.SubtitleEnabled?` _ascustom_game_instance)
        (`self.DialogueCreate`)
        (if (not (`self.WidgetAnimBool`))
          (set `self.WidgetAnimBool` true)
          (`self.GetLineFinal`))))))

(event `self.Box.OnComponentEndOverlap`
  (params (OverlappedComponent :type "PrimitiveComponent Object Reference") (OtherActor :type "Actor Object Reference") (OtherComp :type "PrimitiveComponent Object Reference") (OtherBodyIndex :type Integer))
  (bind _dialoguewidget (`self.DialogueWidget`))
  ;[1 1 1] End Overlap to Remove Dialogue Widget
  (cast `/Game/Hou/Blueprints/BP_PlayerCharacter` OtherActor)
  (if (`self.PreventSubDuplicate`)
    (set `self.PreventSubDuplicate` false)
    (`/Game/Siang/Dialogue/DialogueWidget.SlideOutAnim` _dialoguewidget)
    (`KismetSystemLibrary.Delay` 0.5)
    (`Widget.RemoveFromParent` _dialoguewidget)
    (set `self.DialogueWidget` null)
    (set `self.LineCurrent` 0)
    (set `self.PreventSubDuplicate` true)
    (set `self.SubtitlesOn` false)
    (`self.AudioFadeOut`)))

(event `CloseTextRender`
  (bind (_direction _newtrack_0) (`Timeline|Timeline_0` :!via `ReverseFromEnd`)
    (:`Update`
      (`MaterialInstanceDynamic.SetScalarParameterValue` (`self.TextRenderDynamicMat`) "TextOpacity" _newtrack_0))))

(event `self.ReceiveTick`
  (params (DeltaSeconds :type "Float (single-precision)"))
  ;[1 1 1] Tick Event to Advance(When SubtitlesOn is true, it will advance every SubInterval seconds)
  (if (`self.DisableBool`)
    (set `self.DisableBool` false)
    (`KismetSystemLibrary.Delay` (`self.SubInterval`))
    (set `self.SubtitlesOn` true)
    (elif (`self.SubtitlesOn`)
      (bind _output_get (set `self.DeltaSeconds` (+ (`self.DeltaSeconds`) DeltaSeconds)))
      (if (>= _output_get (`self.SubInterval`))
        (set `self.DeltaSeconds` 0.0)
        (`self.SubtitleInteract`)))))

(event `self.Box.OnComponentBeginOverlap`
  (params (OverlappedComponent :type "PrimitiveComponent Object Reference") (OtherActor :type "Actor Object Reference") (OtherComp :type "PrimitiveComponent Object Reference") (OtherBodyIndex :type Integer) (bFromSweep :type Boolean) (SweepResult :type "HitResult Structure (by ref)"))
  ;[1 1 1] Begin Overlap to Trigger Opening Subtitles
  (if (== OtherActor (`GameplayStatics.GetPlayerCharacter` 0))
    (`/Engine/EditorBlueprintResources/StandardMacros.IsValid` (`self.DialogueWidget`)
      (:`Is Not Valid`
        (`self.SubtitleInteract`)
        (set `self.SubtitlesOn` true)
        (if (`self.FinishedPuzzle`)
          (`self.PlayClosingCue`)
          (else
            (`self.PlayOpeningCue`)))))))

(fn `DialogueCreate`
  (`/Engine/EditorBlueprintResources/StandardMacros.IsValid` (`self.DialogueWidget`)
    (:`Is Valid`
      (bind _returnedline (`self.DialogueGetLine`))
      (set `/Game/Siang/Dialogue/DialogueWidget.DialogueText` _returnedline (`self.DialogueWidget`)))
    (:`Is Not Valid`
      (bind _returnvalue (`|CreateWidget` "/Game/Siang/Dialogue/DialogueWidget.DialogueWidget_C" (`GameplayStatics.GetPlayerController` 0)))
      (bind _output_get (set `self.DialogueWidget` _returnvalue))
      (`UserWidget.AddToViewport` _output_get 0)
      (bind _returnedline_2 (`self.DialogueGetLine`))
      (set `/Game/Siang/Dialogue/DialogueWidget.DialogueText` _returnedline_2 (`self.DialogueWidget`)))))

(fn `DialogueEnable`
  (params (Actor :type "Actor Object Reference") (ConversationID :type Integer) (DeltaSec :type "Float (double-precision)"))
  (set `self.CallerRef` Actor)
  (set `self.Conversation_ID` ConversationID)
  (set `self.DeltaSeconds` DeltaSec)
  (set `self.DisableBool` false)
  (set `self.LineCurrent` 0)
  (set `self.SubtitlesOn` true)
  (`self.SubtitleInteract`))

(fn `DialogueGetLine`
  (returns (ReturnedLine :type Text))
  (locals (ReturnedLines :type "Array of Text"))
  (bind _returnedlines (`local.ReturnedLines`))
  (for _array_element (`self.MyDialogue`)
    (bind _returnvalue (`|GetDataTableRow` (`self.DialogueDataTable`) _array_element)
      (:`then`
        (bind (_npc_id _conversation_id _line_id _dialogue) (break `/Game/Siang/Dialogue/DialogueStructure` _returnvalue))
        (if (and (== _conversation_id (`self.Conversation_ID`)) (== _line_id (`self.LineCurrent`)))
          (`KismetArrayLibrary.Array_Add` _returnedlines _dialogue)))))
  (if (== (`KismetArrayLibrary.Array_Length` _returnedlines) 1)
    (return (`|GetArrayItem` _returnedlines))
    (else
      (set `self.WidgetAnimBool` false))))

(fn `UserConstructionScript`)