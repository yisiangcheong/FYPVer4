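; Interactable piano that plays a 2D sound each time it is interacted with.
; Each interaction plays the current SoundArray entry, then advances ArrayIndex, wrapping it to zero after a hard-coded limit instead of the array length.
; GetInteractionStatus always reports the same fixed status.
; An alternative path that switches, fades and replays an Audio component is left disconnected and never runs.
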(event `/Game/Hou/Blueprints/Interface_Interaction.OnInteracted`
  (bind _arrayindex (`self.ArrayIndex`))
  (`GameplayStatics.PlaySound2D` (`|GetArrayItem` (`self.SoundArray`) _arrayindex) 1.0 1.0 0.0 null null)
  (bind _result (`/Engine/EditorBlueprintResources/StandardMacros.IncrementInt` _arrayindex)
    (:`  `
      (if (> _result 3)
        (set `self.ArrayIndex` 0)))))

(fn `GetInteractionStatus`
  (returns (`Interaction Status` :type "/Game/Hou/Blueprints/Enum_InteractionStatus Enum"))
  (return "NewEnumerator1"))

(fn `UserConstructionScript`)