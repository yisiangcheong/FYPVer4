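; Memory container actor that reveals and hides a room's memory scene through a growing or shrinking sphere.
; BeginPlay gathers Interactable actors inside its box, disables their collision and writes the sphere's location to per-room Material Parameter Collection values.
; ToggleMemory shows the actors, fades a post-process whiteness and expands the sphere, or reverses the timeline to hide them.
; Tick feeds the changing sphere radius into the collection to drive cutoff materials.
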(event `DisableMemoryCollisions`
  (bind _memoryactors (`self.MemoryActors`))
  ;[1 1 1] Disable Memory Model Collisions(After solving)
  (if (> (`KismetArrayLibrary.Array_Length` _memoryactors) 0)
    (for _array_element _memoryactors
      (`self.SetActorEnableCollision` _array_element false))))

(event `self.ReceiveTick`
  (params (DeltaSeconds :type "Float (single-precision)"))
  (bind _returnvalue_x (`KismetMathLibrary.BreakVector` (`SceneComponent.K2_GetComponentScale` (`self.Sphere`))))
  (bind _returnvalue (* _returnvalue_x (`self.SphereRadiusDefaultVal`)))
  ;[1 1 1] Tick Event to set sphere scale
  (if (not (`self.SphereFullyOpened/Closed`))
    (switch `name` (`self.MemoryLocationName`)
      (:`Default`
        (`KismetMaterialLibrary.SetScalarParameterValue` "/Game/Siang/DissolveMaterials/Mat_ParameterCollection_Location.Mat_ParameterCollection_Location" "Radius" _returnvalue))
      (:`Bedroom`
        (`KismetMaterialLibrary.SetScalarParameterValue` "/Game/Siang/DissolveMaterials/Mat_ParameterCollection_Location.Mat_ParameterCollection_Location" "RadiusBedroom" _returnvalue))
      (:`Kitchen`
        (`KismetMaterialLibrary.SetScalarParameterValue` "/Game/Siang/DissolveMaterials/Mat_ParameterCollection_Location.Mat_ParameterCollection_Location" "RadiusKitchen" _returnvalue))
      (:`Toilet`
        (`KismetMaterialLibrary.SetScalarParameterValue` "/Game/Siang/DissolveMaterials/Mat_ParameterCollection_Location.Mat_ParameterCollection_Location" "RadiusToilet" _returnvalue))
      (:`KidRoom`
        (`KismetMaterialLibrary.SetScalarParameterValue` "/Game/Siang/DissolveMaterials/Mat_ParameterCollection_Location.Mat_ParameterCollection_Location" "RadiusKidRoom" _returnvalue))
      (:`LivingRoom`
        (`KismetMaterialLibrary.SetScalarParameterValue` "/Game/Siang/DissolveMaterials/Mat_ParameterCollection_Location.Mat_ParameterCollection_Location" "RadiusLivingRoom" _returnvalue))
      (:`LivingRoom2`
        (`KismetMaterialLibrary.SetScalarParameterValue` "/Game/Siang/DissolveMaterials/Mat_ParameterCollection_Location.Mat_ParameterCollection_Location" "RadiusLivingRoom2" _returnvalue)))))

(event `self.ReceiveBeginPlay`
  (bind _returnvalue (`SceneComponent.K2_GetComponentLocation` (`self.Sphere`)))
  ;[1 1 1] Begin Play, Add Interactable Actors to array, Set Cutoff Material Location
  (for _array_element (`PrimitiveComponent.GetOverlappingActors` (`self.Box`) null)
    (if (`self.ActorHasTag` _array_element "Interactable")
      (`KismetArrayLibrary.Array_Add` (`self.MemoryActors`) _array_element)))
  (`self.DisableMemoryCollisions`)
  (switch `name` (`self.MemoryLocationName`)
    (:`Default`
      (`KismetMaterialLibrary.SetVectorParameterValue` "/Game/Siang/DissolveMaterials/Mat_ParameterCollection_Location.Mat_ParameterCollection_Location" "Location" (`KismetMathLibrary.Conv_VectorToLinearColor` _returnvalue)))
    (:`Bedroom`
      (`KismetMaterialLibrary.SetVectorParameterValue` "/Game/Siang/DissolveMaterials/Mat_ParameterCollection_Location.Mat_ParameterCollection_Location" "LocationBedroom" (`KismetMathLibrary.Conv_VectorToLinearColor` _returnvalue)))
    (:`Kitchen`
      (`KismetMaterialLibrary.SetVectorParameterValue` "/Game/Siang/DissolveMaterials/Mat_ParameterCollection_Location.Mat_ParameterCollection_Location" "LocationKitchen" (`KismetMathLibrary.Conv_VectorToLinearColor` _returnvalue))
      (`PrimitiveComponent.SetCollisionProfileName` (`self.Box`) "OverlapAllDynamic"))
    (:`Toilet`
      (`KismetMaterialLibrary.SetVectorParameterValue` "/Game/Siang/DissolveMaterials/Mat_ParameterCollection_Location.Mat_ParameterCollection_Location" "LocationToilet" (`KismetMathLibrary.Conv_VectorToLinearColor` _returnvalue)))
    (:`KIdRoom`
      (`KismetMaterialLibrary.SetVectorParameterValue` "/Game/Siang/DissolveMaterials/Mat_ParameterCollection_Location.Mat_ParameterCollection_Location" "LocationKidRoom" (`KismetMathLibrary.Conv_VectorToLinearColor` _returnvalue)))
    (:`LivingRoom`
      (`KismetMaterialLibrary.SetVectorParameterValue` "/Game/Siang/DissolveMaterials/Mat_ParameterCollection_Location.Mat_ParameterCollection_Location" "LocationLivingRoom" (`KismetMathLibrary.Conv_VectorToLinearColor` _returnvalue)))
    (:`LivingRoom2`
      (`KismetMaterialLibrary.SetVectorParameterValue` "/Game/Siang/DissolveMaterials/Mat_ParameterCollection_Location.Mat_ParameterCollection_Location" "LocationLivingRoom2" (`KismetMathLibrary.Conv_VectorToLinearColor` _returnvalue)))))

(event `FirstInteract`
  (if (not (`self.PlayedOpeningClue`))
    (set `self.PlayedOpeningClue` true)
    (`self.ToggleMemory`)))

(event `ExpandSphereEvent`
  ;[1 1 1] Sphere Timeline
  (bind (_direction _linear) (`Timeline|Linear` :!label _label)
    (:`Update`
      (`SceneComponent.SetWorldScale3D` (`self.Sphere`) (`KismetMathLibrary.Conv_DoubleToVector` (* _linear (`self.SphereScale`)))))
    (:`Finished`
      (if (`self.SetActive`)
        (set `self.SetActive` false)
        (set `self.SphereFullyOpened/Closed` true)
        (else
          (for _array_element (`self.MemoryActors`)
            (`self.SetActorHiddenInGame` _array_element true)
            (`self.SetActorEnableCollision` _array_element false))
          (set `self.SetActive` true)
          (set `PostProcessComponent.bEnabled` false (`self.PostProcess`))
          (set `self.SphereFullyOpened/Closed` true))))))

(event `self.Box.OnComponentBeginOverlap`
  (params (OverlappedComponent :type "PrimitiveComponent Object Reference") (OtherActor :type "Actor Object Reference") (OtherComp :type "PrimitiveComponent Object Reference") (OtherBodyIndex :type Integer) (bFromSweep :type Boolean) (SweepResult :type "HitResult Structure (by ref)"))
  ;[1 1 1] Begin Overlap
  (if (== OtherActor (`GameplayStatics.GetPlayerCharacter` 0))
    _))

(event `ShrinkSphereEvent`
  ;[1 1 1] Sphere Timeline
  (goto _label :!via `ReverseFromEnd`))

(event `ToggleMemory`
  ;[1 1 1] ToggleMemory Custom event
  (if (`self.SetActive`)
    (for _array_element (`self.MemoryActors`)
      (`self.SetActorHiddenInGame` _array_element false)
      (`self.SetActorEnableCollision` _array_element true))
    (set `PostProcessComponent.bEnabled` true (`self.PostProcess`))
    (`|ExecutionSequence`
      (:`then_0`
        (bind (_direction _white) (`Timeline|PPM_Whiteness` :!via `PlayFromStart`)
          (:`Update`
            (`KismetMaterialLibrary.SetScalarParameterValue` "/Game/Siang/DissolveMaterials/Mat_ParameterCollection_Location.Mat_ParameterCollection_Location" "PPM_Whiteness" _white))))
      (:`then_1`
        (`KismetSystemLibrary.Delay` 0.5)
        (`self.ExpandSphere`)
        (set `self.SphereFullyOpened/Closed` false)))
    (else
      (`self.ShrinkSphere`)
      (set `self.SphereFullyOpened/Closed` false)
      (`PrimitiveComponent.SetCollisionEnabled` (`self.Box`) "NoCollision"))))

(fn `Close`
  (`self.ToggleMemory`))

(fn `ExpandSphere`
  (`self.ExpandSphereEvent`)
  (`KismetSystemLibrary.PrintString` "EXPAND"))

(fn `ShrinkSphere`
  (`self.ShrinkSphereEvent`)
  (`KismetSystemLibrary.PrintString` "SHRINK"))

(fn `UserConstructionScript`)