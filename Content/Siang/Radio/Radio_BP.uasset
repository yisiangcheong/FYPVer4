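; Radio tuning puzzle: the player possesses the radio through a camera lerp and scrolls the mouse wheel to find the right station.
; The wheel moves knob and needle, whose distance from four channel positions sets audio channel and static, with playback synced to elapsed time.
; Tuning in the correct channel starts a dialogue, whose end restores player control and plays closing dialogue.
; The radio then hides, closes its memory portal and reveals subsequent memory items.
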(event `self.ReceiveBeginPlay`
  (bind _audio (`self.Audio`))
  ;[1 1 1] Begin Play
  (set `self.CameraOriPos` (`SceneComponent.K2_GetComponentToWorld` (`self.Camera`)))
  (`self.SetActorEnableCollision` (`self.SubtitleActor`) false)
  (for _array_element (`self.SubsequentParticleEmitters`)
    (`ActorComponent.Deactivate` (`Emitter.ParticleSystemComponent` _array_element)))
  (`AudioComponent.Play` _audio 0.0)
  (`AudioComponent.AdjustVolume` _audio 0.0 0.1)
  (set `self.RadioNoise` 100.0)
  (`AudioComponent.SetFloatParameter` (`self.Audio`) "RadioFloat" (`self.RadioNoise`))
  (for _array_element_2 (`self.SubsequentSubtitleBPs`)
    (`self.SetActorEnableCollision` _array_element_2 false))
  (for _array_element_3 (`self.SubsequentMemoryItems`)
    (`self.SetActorEnableCollision` _array_element_3 false)
    (`self.SetActorHiddenInGame` _array_element_3 true)
    (for _array_element_4 (`self.GetAllChildActors` _array_element_3 true)
      (`self.SetActorEnableCollision` _array_element_4 false)
      (`self.SetActorHiddenInGame` _array_element_4 true))))

(event `InputAxisKey|MouseWheelAxis`
  (params (AxisValue :type "Float (single-precision)"))
  (bind (_inrange_ _difference) (`self.CalculateChannelGap` -12.5))
  (bind (_inrange__2 _difference_2) (`self.CalculateChannelGap` 20.0))
  (bind (_inrange__3 _difference_3) (`self.CalculateChannelGap` 10.0))
  (bind (_inrange__4 _difference_4) (`self.CalculateChannelGap` -1.5))
  (bind _audio (`self.Audio`))
  (bind _returnvalue (* AxisValue (`self.KnobSensitivity`)))
  (bind _relativelocation_x (`KismetMathLibrary.BreakVector` (`SceneComponent.RelativeLocation` (`self.needle_pivot`))))
  ;[1 1 1] Mouse Wheel Input
  (if (or (and (< AxisValue 0.0) (< _relativelocation_x (`self.StickMaxX`))) (and (> AxisValue 0.0) (> _relativelocation_x (`self.StickMinX`))))
    (`SceneComponent.K2_AddLocalRotation` (`self.knob_pivot`) (`KismetMathLibrary.MakeRotator` 0.0 _returnvalue) false false)
    (`SceneComponent.K2_AddRelativeLocation` (`self.needle_pivot`) (`KismetMathLibrary.MakeVector` (* _returnvalue -0.2)) false false)
    (if _inrange__2
      (`AudioComponent.SetIntParameter` (`self.Audio`) "Channel" 3)
      (set `self.RadioNoise` (* (/ _difference_2 (`self.ChannelGapTolerance`)) 100.0))
      (`AudioComponent.Play` _audio (mod (`self.TimeElapsed`) (`SoundBase.Duration` (`AudioComponent.Sound` _audio))) :!label _label)
      (`AudioComponent.SetFloatParameter` (`self.Audio`) "RadioFloat" (`self.RadioNoise`) :!label _label_2)
      (elif _inrange__3
        (`AudioComponent.SetIntParameter` (`self.Audio`) "Channel" 2)
        (set `self.RadioNoise` (* (/ _difference_3 (`self.ChannelGapTolerance`)) 100.0))
        (goto _label)
        (elif _inrange__4
          (`AudioComponent.SetIntParameter` (`self.Audio`) "Channel" 1)
          (set `self.RadioNoise` (* (/ _difference_4 (`self.ChannelGapTolerance`)) 100.0))
          (goto _label)
          (elif _inrange_
            (`AudioComponent.SetIntParameter` (`self.Audio`) "Channel" 0)
            (set `self.RadioNoise` (* (/ _difference (`self.ChannelGapTolerance`)) 100.0))
            (`AudioComponent.SetFloatParameter` (`self.Audio`) "RadioFloat" (`self.RadioNoise`))
            (if (and (<= (`self.RadioNoise`) 25.0) (not (`self.Win?`)))
              (`/Game/Siang/Dialogue/Subtitle_BP.DialogueEnable` (`self.SubtitleActor`) self 3 0.0)
              (`AudioComponent.Play` (`self.Audio`) 0.0))
            (else
              (set `self.RadioNoise` 100.0)
              (goto _label_2))))))))

(event `/Game/Hou/Blueprints/Interface_Interaction.OnInteracted`
  (bind _returnvalue (`GameplayStatics.GetPlayerController` 0))
  (if (`self.FirstInteract`)
    ;[1 1 1] On Interacted Event
    (if (`self.CanBeInteracted`)
      (set `self.PlayerCamOriPos` (`SceneComponent.K2_GetComponentToWorld` (`PlayerCameraManager.TransformComponent` (`GameplayStatics.GetPlayerCameraManager` 0))))
      (`AudioComponent.AdjustVolume` (`self.Audio`) 0.0 1.0)
      (`AudioComponent.AdjustVolume` (`self.RadioSoundCueReverse`) 0.0 0.0)
      (set `self.PlayerPawnReference` (`Controller.K2_GetPawn` (`GameplayStatics.GetPlayerController` 0)))
      (`Controller.Possess` _returnvalue self)
      ;[1 1 1] Camera Lerp
      (bind (_direction _lerpfloat) (`Timeline|CameraLerpTimeline` :!via `PlayFromStart`)
        (:`Update`
          (`SceneComponent.K2_SetWorldTransform` (`self.Camera`) (`KismetMathLibrary.TLerp` (`SceneComponent.K2_GetComponentToWorld` (`PlayerCameraManager.TransformComponent` (`GameplayStatics.GetPlayerCameraManager` 0))) (`self.CameraOriPos`) _lerpfloat) false false))
        (:`Finished`
          (set `PlayerController.bShowMouseCursor` true _returnvalue)
          ;[1 1 1] Alex's Book Disabled
          (bind _asnew_player_controller (cast `/Game/Alex/NewPlayerController` (`GameplayStatics.GetPlayerController` 0)))
          (set `/Game/Alex/NewPlayerController.InPuzzle` true _asnew_player_controller))))
    (else
      (set `self.FirstInteract` true)
      (`/Game/Siang/ItemClass/MemoryContainer_BP.FirstInteract` (`self.MemoryPortal`))
      (`self.SetActorEnableCollision` (`self.SubtitleActor`) true))))

(event `self.ReceiveTick`
  (params (DeltaSeconds :type "Float (single-precision)"))
  ;[1 1 1] Tick Event
  (set `self.TimeElapsed` (+ (`self.TimeElapsed`) DeltaSeconds)))

(event `Key|Escape`
  (params (Key :type "Key Structure"))
  ;[1 1 1] Esc to Exit Puzzle
  (:`Pressed`
    ;[1 1 1] Camera Lerp Reverse
    (bind (_direction _lerpfloat) (`Timeline|Timeline_1` :!via `ReverseFromEnd`)
      (:`Update`
        (`SceneComponent.K2_SetWorldTransform` (`self.Camera`) (`KismetMathLibrary.TLerp` (`self.PlayerCamOriPos`) (`self.CameraOriPos`) _lerpfloat) false false))
      (:`Finished`
        (`self.ExitRadioPuzzle`)))))

(event `self.ClosingClues.OnAudioFinished`
  ;[1 1 1] On Audio Finished
)

(event `/Game/Hou/Blueprints/Interface_PuzzleUpdate.OnDialogueFinished`
  (bind _subtitleactor (`self.SubtitleActor`))
  (bind _completedpuzzles (`self.CompletedPuzzles`))
  ;[1 1 1] Radio Solved
  (if (and (`self.Win?`) (== (`/Game/Siang/Dialogue/Subtitle_BP.Conversation_ID` (`self.SubtitleActor`)) (`self.SubtitleLastConvoID`)))
    (message `/Game/Hou/Blueprints/Interface_PuzzleUpdate.OnClosingClueEnded` (`self.PlayerPawnReference`) "NewEnumerator1")
    (`/Game/Siang/Dialogue/Subtitle_BP.AudioFadeOut` (`self.SubtitleActor`))
    (`ActorComponent.Deactivate` (`Emitter.ParticleSystemComponent` (`self.ParticleEmitterRadio`)))
    (`/Game/Siang/Dialogue/Subtitle_BP.CloseTextRender` (`self.SubtitleActor`))
    (for _array_element (`self.SubsequentParticleEmitters`)
      (`ActorComponent.Activate` (`Emitter.ParticleSystemComponent` _array_element) false))
    (`/Game/Siang/ItemClass/MemoryContainer_BP.Close` (`self.MemoryPortal`))
    (`self.SetActorEnableCollision` false)
    (`self.SetActorHiddenInGame` true)
    (set `/Game/Siang/CompletedPuzzles_BP.CompletedPuzzlesInt` (+ (`/Game/Siang/CompletedPuzzles_BP.CompletedPuzzlesInt` _completedpuzzles) 1) _completedpuzzles)
    (for _array_element_2 (`self.SubsequentMemoryContainers`)
      (`PrimitiveComponent.SetCollisionProfileName` (`/Game/Siang/ItemClass/MemoryContainer_BP.Box` _array_element_2) "OverlapAllDynamic"))
    (for _array_element_3 (`self.SubsequentMemoryItems`)
      (`self.SetActorHiddenInGame` _array_element_3 false)
      (`self.SetActorEnableCollision` _array_element_3 true)
      (for _array_element_4 (`self.GetAllChildActors` _array_element_3 true)
        (`self.SetActorHiddenInGame` _array_element_4 false)
        (`self.SetActorEnableCollision` _array_element_4 true)))
    (elif (== (`/Game/Siang/Dialogue/Subtitle_BP.Conversation_ID` (`self.SubtitleActor`)) 3)
      (set `self.CanBeInteracted` false)
      (set `self.Win?` true)
      (`KismetSystemLibrary.Delay` 0.0)
      (`AudioComponent.SetFloatParameter` (`self.Audio`) "RadioFloat" (`self.RadioNoise`))
      ;[1 1 1] Camera Lerp Reverse
      (bind (_direction _lerpfloat) (`Timeline|Timeline_0` :!via `ReverseFromEnd`)
        (:`Update`
          (`SceneComponent.K2_SetWorldTransform` (`self.Camera`) (`KismetMathLibrary.TLerp` (`self.PlayerCamOriPos`) (`self.CameraOriPos`) _lerpfloat) false false))
        (:`Finished`
          (`KismetSystemLibrary.Delay` 3.0)
          (`self.ExitRadioPuzzle`)
          (bind _asnew_player_controller (cast `/Game/Alex/NewPlayerController` (`GameplayStatics.GetPlayerController` 0)))
          (set `/Game/Alex/NewPlayerController.InPuzzle` false _asnew_player_controller)
          (`/Game/Siang/Dialogue/Subtitle_BP.DialogueEnable` (`self.SubtitleActor`) self (`self.SubtitleLastConvoID`) 0.0)
          (`AudioComponent.AdjustVolume` (`self.Audio`) 3.0 0.0)
          (`/Game/Siang/Dialogue/Subtitle_BP.PlayClosingCue` _subtitleactor)
          (set `/Game/Siang/Dialogue/Subtitle_BP.FinishedPuzzle` true _subtitleactor))))))

(fn `ExitRadioPuzzle`
  (bind _returnvalue (`GameplayStatics.GetPlayerController` 0))
  (`Controller.Possess` _returnvalue (`self.PlayerPawnReference`))
  (set `PlayerController.bShowMouseCursor` false _returnvalue)
  (`WidgetBlueprintLibrary.SetInputMode_GameOnly` _returnvalue)
  (set `PlayerController.bEnableMouseOverEvents` false _returnvalue)
  (`MaterialInstanceDynamic.SetScalarParameterValue` (`self.MatInstanceDynamic`) "TimeMultiply" 3.0))

(fn `UserConstructionScript`)