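; SphereMasker_BP is a sphere actor that drives dissolve materials by publishing its position and size to a material parameter collection.
; The construction script and Tick write the sphere's world location to Location, and its X world scale times a default radius to Radius.
; Timelines meant to expand or shrink the actor's scale exist but are unconnected, and the Expand and Shrink functions are empty.
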(event `self.ReceiveBeginPlay`)

(event `self.ReceiveTick`
  (params (DeltaSeconds :type "Float (single-precision)"))
  (bind _returnvalue_x (`KismetMathLibrary.BreakVector` (`SceneComponent.K2_GetComponentScale` (`self.Sphere`))))
  (`KismetMaterialLibrary.SetVectorParameterValue` "/Game/Siang/DissolveMaterials/Mat_ParameterCollection_Location.Mat_ParameterCollection_Location" "Location" (`KismetMathLibrary.Conv_VectorToLinearColor` (`SceneComponent.K2_GetComponentLocation` (`self.Sphere`))))
  (`KismetMaterialLibrary.SetScalarParameterValue` "/Game/Siang/DissolveMaterials/Mat_ParameterCollection_Location.Mat_ParameterCollection_Location" "Radius" (* _returnvalue_x (`self.RadiusDefaultVal`))))

(fn `Expand`)

(fn `Shrink`)

(fn `UserConstructionScript`
  (bind _returnvalue_x (`KismetMathLibrary.BreakVector` (`SceneComponent.K2_GetComponentScale` (`self.Sphere`))))
  (`KismetMaterialLibrary.SetVectorParameterValue` "/Game/Siang/DissolveMaterials/Mat_ParameterCollection_Location.Mat_ParameterCollection_Location" "Location" (`KismetMathLibrary.Conv_VectorToLinearColor` (`SceneComponent.K2_GetComponentLocation` (`self.Sphere`))))
  (`KismetMaterialLibrary.SetScalarParameterValue` "/Game/Siang/DissolveMaterials/Mat_ParameterCollection_Location.Mat_ParameterCollection_Location" "Radius" (* _returnvalue_x (`self.RadiusDefaultVal`))))